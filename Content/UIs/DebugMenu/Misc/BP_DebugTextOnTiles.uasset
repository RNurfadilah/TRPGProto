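; Debug actor that shows X,Y index labels above the walkable tiles of BP_Grid when ShowTileIndexes is on.
; On BeginPlay it finds the grid and binds to its tile-updated and grid-destroyed events.
; Labels are TextRenderActors spawned on demand with tick off and cached in a map by tile index for reuse.
; Updates remove labels for missing or non-walkable tiles, and toggling the flag rebuilds or clears all labels.
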(event `self.ReceiveBeginPlay`
  (bind _returnvalue (`GameplayStatics.GetActorOfClass` "/Game/Blueprints/Cores/Grid/BP_Grid.BP_Grid_C"))
  (bind _output_get (set `self.Grid` _returnvalue))
  (add `/Game/Blueprints/Cores/Grid/BP_Grid.OnTileDataUpdated` _output_get (`|CreateDelegate` :!event `UpdateTextOnTile`))
  (add `/Game/Blueprints/Cores/Grid/BP_Grid.OnGridDestroyed` _output_get (`|CreateDelegate` :!event `ClearAllTextActor`)))

(fn `ClearAllTextActor`
  (bind _spawntexts (`self.SpawnTexts`))
  (bind _values (`BlueprintMapLibrary.Map_Values` _spawntexts))
  (for _array_element _values
    (`self.K2_DestroyActor` _array_element))
  (`BlueprintMapLibrary.Map_Clear` _spawntexts))

(fn `DestroyTextActor`
  (params (Index :type "IntPoint Structure"))
  (locals (Actor :type "TextRenderActor Object Reference"))
  (bind _output_get (set `local.Actor` (`BlueprintMapLibrary.Map_Find` (`self.SpawnTexts`) Index)))
  (`/Engine/EditorBlueprintResources/StandardMacros.IsValid` _output_get
    (:`Is Valid`
      (`self.K2_DestroyActor`)
      (`BlueprintMapLibrary.Map_Remove` (`self.SpawnTexts`) (`local.Index`)))))

(fn `GetTextActor`
  (params (Index :type "IntPoint Structure"))
  (returns (TextRenderActor :type "TextRenderActor Object Reference"))
  (locals (Actor :type "TextRenderActor Object Reference"))
  (bind _textrender (`TextRenderActor.TextRender` (`local.Actor`)))
  (bind _output_get (set `local.Actor` (`BlueprintMapLibrary.Map_Find` (`self.SpawnTexts`) Index)))
  (`/Engine/EditorBlueprintResources/StandardMacros.IsValid` _output_get
    (:`Is Valid`
      (return (`local.Actor`)))
    (:`Is Not Valid`
      (bind _returnvalue (`|SpawnActorFromClass` "/Script/Engine.TextRenderActor" (`KismetMathLibrary.MakeTransform` (0.0 0.0 0.0)) "AlwaysSpawn" "OverrideRootScale" null null))
      (set `local.Actor` _returnvalue)
      (`BlueprintMapLibrary.Map_Add` (`self.SpawnTexts`) (`local.Index`) (`local.Actor`))
      (`self.SetActorTickEnabled` (`local.Actor`) false)
      (`self.SetActorEnableCollision` false)
      (`TextRenderComponent.SetHorizontalAlignment` _textrender "EHTA_Center")
      (`TextRenderComponent.SetVerticalAlignment` _textrender "EVRTA_TextCenter")
      (return (`local.Actor`)))))

(fn `SetShowTileIndexes`
  (params (ShowTileIndexes :type Boolean))
  (bind _output_get (set `self.Show Tile Indexes` ShowTileIndexes))
  (if _output_get
    (bind _keys (`BlueprintMapLibrary.Map_Keys` (`/Game/Blueprints/Cores/Grid/BP_Grid.GridTiles` (`self.Grid`))))
    (for _array_element _keys
      (`self.UpdateTextOnTile` _array_element))
    (else
      (`self.ClearAllTextActor`))))

(fn `UpdateTextOnTile`
  (params (Index :type "IntPoint Structure"))
  (locals (Data :type "/Game/Blueprints/Cores/Utility/S_TileData Structure") (TextActor :type "TextRenderActor Object Reference") (Text :type String))
  (bind (_data_index _data_tiletype) (break `/Game/Blueprints/Cores/Utility/S_TileData` (`local.Data`)))
  (bind (_index_x _index_y) (break `IntPoint` (`local.Index`)))
  (bind (_value _returnvalue) (`BlueprintMapLibrary.Map_Find` (`/Game/Blueprints/Cores/Grid/BP_Grid.GridTiles` (`self.Grid`)) (`local.Index`)))
  (if (`self.Show Tile Indexes`)
    (if _returnvalue
      (set `local.Data` _value)
      (if (`/Game/Blueprints/Cores/Utility/BFL_TileData.IsTileTypeWalkAble` _data_tiletype)
        (bind _textrenderactor (`self.GetTextActor` (`local.Index`)))
        (set `local.TextActor` _textrenderactor)
        (set `local.Text` (`KismetStringLibrary.Concat_StrStr` (`KismetStringLibrary.Conv_IntToString` _index_x) ", " (`KismetStringLibrary.Conv_IntToString` _index_y)))
        (`TextRenderComponent.K2_SetText` (`TextRenderActor.TextRender` (`local.TextActor`)) (`KismetTextLibrary.Conv_StringToText` (`local.Text`)))
        (`self.K2_SetActorTransform` (`local.TextActor`) (`KismetMathLibrary.MakeTransform` (+ (.location (`.Transform_8_1A7B87B34336F36EDDECB69D5BF0102F` (break `/Game/Blueprints/Cores/Utility/S_TileData` (`local.Data`)))) (0.0 0.0 1.0)) (struct :`Pitch` 90.0 :`Yaw` 180.0) (2.0 2.0 2.0)) false false)
        (else
          (`self.DestroyTextActor` (`local.Index`) :!label _label)))
      (else
        (goto _label)))))

(fn `UserConstructionScript`)