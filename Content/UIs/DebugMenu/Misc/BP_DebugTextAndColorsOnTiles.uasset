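; Debug actor that visualizes grid and pathfinding data on the tiles of BP_Grid.
; Toggleable text for tile indexes, pathfinding costs and sort order uses TextRenderActors, spawned on demand per walkable tile, cached by index and scaled to the longest entry.
; Discovered and analyzed tiles are marked by adding or removing grid tile states.
; BeginPlay binds to grid and pathfinding delegates, while setter functions refresh all tiles when display options change.
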(event `self.ReceiveBeginPlay`
  (bind _gridpathfinding (`/Game/Blueprints/Cores/Grid/BP_Grid.GridPathFinding` (`self.Grid`)))
  (bind _gridpathfinding_2 (`/Game/Blueprints/Cores/Grid/BP_Grid.GridPathFinding` (`self.Grid`)))
  (bind _returnvalue (`GameplayStatics.GetActorOfClass` "/Game/Blueprints/Cores/Grid/BP_Grid.BP_Grid_C"))
  (bind _output_get (set `self.Grid` _returnvalue))
  (add `/Game/Blueprints/Cores/Grid/BP_Grid.OnTileDataUpdated` _output_get (`|CreateDelegate` :!event `UpdateTextOnTile`))
  (add `/Game/Blueprints/Cores/Grid/BP_Grid.OnGridDestroyed` _output_get (`|CreateDelegate` :!event `ClearAllTextActor`))
  (add `/Game/Blueprints/Cores/Grid/BP_GridPathFinding.OnPathFindingDataUpdated` _gridpathfinding_2 (`|CreateDelegate` :!event `UpdateStateOnTiles`))
  (add `/Game/Blueprints/Cores/Grid/BP_GridPathFinding.OnPathFindingDataCleared` _gridpathfinding_2 (`|CreateDelegate` :!event `UpdateStateOnAllTiles`))
  (add `/Game/Blueprints/Cores/Grid/BP_GridPathFinding.OnPathFindingDataUpdated` _gridpathfinding (`|CreateDelegate` :!event `UpdateTextOnTile`))
  (add `/Game/Blueprints/Cores/Grid/BP_GridPathFinding.OnPathFindingDataCleared` _gridpathfinding (`|CreateDelegate` :!event `UpdateTextOnAllTiles`)))

(fn `ClearAllTextActor`
  (bind _spawntexts (`self.SpawnTexts`))
  (bind _values (`BlueprintMapLibrary.Map_Values` _spawntexts))
  (for _array_element _values
    (`self.K2_DestroyActor` _array_element))
  (`BlueprintMapLibrary.Map_Clear` _spawntexts))

(fn `DestroyTextActor`
  (params (Index :type "IntPoint Structure"))
  (locals (Actor :type "TextRenderActor Object Reference"))
  (bind _output_get (set `local.Actor` (`BlueprintMapLibrary.Map_Find` (`self.SpawnTexts`) Index)))
  (`/Engine/EditorBlueprintResources/StandardMacros.IsValid` _output_get
    (:`Is Valid`
      (`self.K2_DestroyActor`)
      (`BlueprintMapLibrary.Map_Remove` (`self.SpawnTexts`) (`local.Index`)))))

(fn `GetTextActor`
  (params (Index :type "IntPoint Structure"))
  (returns (TextRenderActor :type "TextRenderActor Object Reference"))
  (locals (Actor :type "TextRenderActor Object Reference"))
  (bind _textrender (`TextRenderActor.TextRender` (`local.Actor`)))
  (bind _output_get (set `local.Actor` (`BlueprintMapLibrary.Map_Find` (`self.SpawnTexts`) Index)))
  (`/Engine/EditorBlueprintResources/StandardMacros.IsValid` _output_get
    (:`Is Valid`
      (return (`local.Actor`)))
    (:`Is Not Valid`
      (bind _returnvalue (`|SpawnActorFromClass` "/Script/Engine.TextRenderActor" (`KismetMathLibrary.MakeTransform` (0.0 0.0 0.0)) "AlwaysSpawn" "OverrideRootScale" null null))
      (set `local.Actor` _returnvalue)
      (`BlueprintMapLibrary.Map_Add` (`self.SpawnTexts`) (`local.Index`) (`local.Actor`))
      (`self.SetActorTickEnabled` (`local.Actor`) false)
      (`self.SetActorEnableCollision` false)
      (`TextRenderComponent.SetHorizontalAlignment` _textrender "EHTA_Center")
      (`TextRenderComponent.SetVerticalAlignment` _textrender "EVRTA_TextCenter")
      (return (`local.Actor`)))))

(fn `SetShowTileStates`
  (params (ShowDiscoveredTiles :type Boolean) (ShowAnalizedTiles :type Boolean))
  (set `self.ShowDiscoveredTiles` ShowDiscoveredTiles)
  (set `self.ShowAnalizedTiles` ShowAnalizedTiles)
  (`self.UpdateStateOnAllTiles`))

(fn `SetShowTileTexts`
  (params (ShowTileIndexes :type Boolean) (ShowCostToEnterTile :type Boolean) (ShowMinCostToTarget :type Boolean) (ShowCostFromStart :type Boolean) (ShowSortOrder :type Boolean))
  (set `self.Show Tile Indexes` ShowTileIndexes)
  (set `self.ShowCostToEnterTile` ShowCostToEnterTile)
  (set `self.ShowMinCostToTarget` ShowMinCostToTarget)
  (set `self.ShowCostFromStart` ShowCostFromStart)
  (set `self.ShowSortOrder` ShowSortOrder)
  (`self.UpdateTextOnAllTiles`))

(fn `UpdateStateOnAllTiles`
  (bind _grid (`self.Grid`))
  (if (or (`self.ShowDiscoveredTiles`) (`self.ShowAnalizedTiles`))
    (bind _keys (`BlueprintMapLibrary.Map_Keys` (`/Game/Blueprints/Cores/Grid/BP_Grid.GridTiles` (`self.Grid`))))
    (for _array_element _keys
      (`self.UpdateStateOnTiles` _array_element))
    (else
      (`/Game/Blueprints/Cores/Grid/BP_Grid.ClearStateFromTiles` _grid "NewEnumerator5")
      (`/Game/Blueprints/Cores/Grid/BP_Grid.ClearStateFromTiles` _grid "NewEnumerator6"))))

(fn `UpdateStateOnTiles`
  (params (Index :type "IntPoint Structure"))
  (`|ExecutionSequence`
    (:`then_0`
      (if (`self.ShowDiscoveredTiles`)
        (if (`KismetArrayLibrary.Array_Contains` (`/Game/Blueprints/Cores/Grid/BP_GridPathFinding.DiscoveredTileIndexes` (`/Game/Blueprints/Cores/Grid/BP_Grid.GridPathFinding` (`self.Grid`))) (`local.Index`))
          (`/Game/Blueprints/Cores/Grid/BP_Grid.AddStateToTile` (`self.Grid`) (`local.Index`) "NewEnumerator5")
          (else
            (`/Game/Blueprints/Cores/Grid/BP_Grid.RemoveStateToTile` (`self.Grid`) (`local.Index`) "NewEnumerator5" :!label _label)))
        (else
          (goto _label))))
    (:`then_1`
      (if (`self.ShowAnalizedTiles`)
        (if (`KismetArrayLibrary.Array_Contains` (`/Game/Blueprints/Cores/Grid/BP_GridPathFinding.AnalizeTileIndexes` (`/Game/Blueprints/Cores/Grid/BP_Grid.GridPathFinding` (`self.Grid`))) (`local.Index`))
          (`/Game/Blueprints/Cores/Grid/BP_Grid.AddStateToTile` (`self.Grid`) (`local.Index`) "NewEnumerator6")
          (else
            (`/Game/Blueprints/Cores/Grid/BP_Grid.RemoveStateToTile` (`self.Grid`) (`local.Index`) "NewEnumerator6" :!label _label_2)))
        (else
          (goto _label_2))))))

(fn `UpdateTextOnAllTiles`
  (if (`self.WantToDisplayAnyText`)
    (bind _keys (`BlueprintMapLibrary.Map_Keys` (`/Game/Blueprints/Cores/Grid/BP_Grid.GridTiles` (`self.Grid`))))
    (for _array_element _keys
      (`self.UpdateTextOnTile` _array_element))
    (else
      (`self.ClearAllTextActor`))))

(fn `UpdateTextOnTile`
  (params (Index :type "IntPoint Structure"))
  (locals (Data :type "/Game/Blueprints/Cores/Utility/S_TileData Structure") (TextActor :type "TextRenderActor Object Reference") (Text :type "Array of String") (PathFindingData :type "/Game/Blueprints/Cores/Utility/S_PathFindingData Structure") (TextLenght :type "Array of Integer"))
  (bind (_data_index _data_tiletype) (break `/Game/Blueprints/Cores/Utility/S_TileData` (`local.Data`)))
  (bind (_index_x _index_y) (break `IntPoint` (`local.Index`)))
  (bind ((`MinimumCostToTarget_13_B80A5E824DB644D421F8229013151D33` _minimumcosttotarget)) (break `/Game/Blueprints/Cores/Utility/S_PathFindingData` (`local.PathFindingData`)))
  (bind ((`CosFromStart_12_3D38642B429114C0012CBDA898A886AF` _cosfromstart)) (break `/Game/Blueprints/Cores/Utility/S_PathFindingData` (`local.PathFindingData`)))
  (bind _gridpathfinding (`/Game/Blueprints/Cores/Grid/BP_Grid.GridPathFinding` (`self.Grid`)))
  (bind (_grid_tile_size_x _grid_tile_size_y) (`KismetMathLibrary.BreakVector` (`/Game/Blueprints/Cores/Grid/BP_Grid.Grid Tile Size` (`self.Grid`))))
  (bind (_value _returnvalue) (`BlueprintMapLibrary.Map_Find` (`/Game/Blueprints/Cores/Grid/BP_Grid.GridTiles` (`self.Grid`)) (`local.Index`)))
  (bind _returnvalue_2 (`KismetStringLibrary.Concat_StrStr` (`KismetStringLibrary.Conv_IntToString` _index_x) ", " (`KismetStringLibrary.Conv_IntToString` _index_y)))
  (bind _returnvalue_3 (`KismetArrayLibrary.Array_Find` (`/Game/Blueprints/Cores/Grid/BP_GridPathFinding.DiscoveredTileIndexes` _gridpathfinding) (`local.Index`)))
  (bind (_value_2 _returnvalue_4) (`BlueprintMapLibrary.Map_Find` (`/Game/Blueprints/Cores/Grid/BP_GridPathFinding.PathFindingData` (`/Game/Blueprints/Cores/Grid/BP_Grid.GridPathFinding` (`self.Grid`))) (`local.Index`)))
  (bind _returnvalue_5 (`KismetStringLibrary.Concat_StrStr` "Enter : " (`KismetStringLibrary.Conv_IntToString` (`.CosToEnterTile_11_5A1FD0B849FD905C9E3A8489915E8F8D` (break `/Game/Blueprints/Cores/Utility/S_PathFindingData` (`local.PathFindingData`))))))
  (bind _returnvalue_6 (`KismetStringLibrary.Concat_StrStr` "Min : " (`KismetStringLibrary.Conv_IntToString` _minimumcosttotarget)))
  (bind _returnvalue_7 (`KismetStringLibrary.Concat_StrStr` "Start : " (`KismetStringLibrary.Conv_IntToString` _cosfromstart)))
  (bind _returnvalue_8 (`KismetStringLibrary.Concat_StrStr` "Sort : " (`KismetStringLibrary.Conv_IntToString` _returnvalue_3) " ( " (`KismetStringLibrary.Conv_IntToString` (`|GetArrayItem` (`/Game/Blueprints/Cores/Grid/BP_GridPathFinding.DiscoveredTileSortingCost` _gridpathfinding) _returnvalue_3)) " ) "))
  (if (`self.WantToDisplayAnyText`)
    (if _returnvalue
      (set `local.Data` _value)
      (if (`/Game/Blueprints/Cores/Utility/BFL_TileData.IsTileTypeWalkAble` _data_tiletype)
        (`|ExecutionSequence`
          (:`then_0`
            (`|ExecutionSequence`
              (:`then_0`
                (if (`self.Show Tile Indexes`)
                  (`KismetArrayLibrary.Array_Add` (`local.Text`) _returnvalue_2)
                  (`KismetArrayLibrary.Array_Add` (`local.TextLenght`) (`KismetStringLibrary.Len` _returnvalue_2))))
              (:`then_1`
                (if (or (`self.ShowCostToEnterTile`) (`self.ShowMinCostToTarget`) (`self.ShowCostFromStart`) (`self.ShowSortOrder`))
                  (if _returnvalue_4
                    (set `local.PathFindingData` _value_2)
                    (`|ExecutionSequence`
                      (:`then_0`
                        (if (`self.ShowCostToEnterTile`)
                          (`KismetArrayLibrary.Array_Add` (`local.Text`) _returnvalue_5)
                          (`KismetArrayLibrary.Array_Add` (`local.TextLenght`) (`KismetStringLibrary.Len` _returnvalue_5))))
                      (:`then_1`
                        (if (`self.ShowMinCostToTarget`)
                          (if (!= _minimumcosttotarget 999999)
                            (`KismetArrayLibrary.Array_Add` (`local.Text`) _returnvalue_6)
                            (`KismetArrayLibrary.Array_Add` (`local.TextLenght`) (`KismetStringLibrary.Len` _returnvalue_6)))))
                      (:`then_2`
                        (if (`self.ShowCostFromStart`)
                          (if (!= _cosfromstart 999999)
                            (`KismetArrayLibrary.Array_Add` (`local.Text`) _returnvalue_7)
                            (`KismetArrayLibrary.Array_Add` (`local.TextLenght`) (`KismetStringLibrary.Len` _returnvalue_7)))))
                      (:`then_3`
                        (if (`self.ShowSortOrder`)
                          (if (!= _returnvalue_3 -1)
                            (`KismetArrayLibrary.Array_Add` (`local.Text`) _returnvalue_8)
                            (`KismetArrayLibrary.Array_Add` (`local.TextLenght`) (`KismetStringLibrary.Len` _returnvalue_8)))))))))))
          (:`then_1`
            (if (> (`KismetArrayLibrary.Array_Length` (`local.Text`)) 0)
              (bind _textrenderactor (`self.GetTextActor` (`local.Index`)))
              (set `local.TextActor` _textrenderactor)
              (`TextRenderComponent.K2_SetText` (`TextRenderActor.TextRender` (`local.TextActor`)) (`KismetTextLibrary.Conv_StringToText` (`KismetStringLibrary.JoinStringArray` (`local.Text`) "  \n")))
              (`self.K2_SetActorTransform` (`local.TextActor`) (`KismetMathLibrary.MakeTransform` (+ (.location (`.Transform_8_1A7B87B34336F36EDDECB69D5BF0102F` (break `/Game/Blueprints/Cores/Utility/S_TileData` (`local.Data`)))) (0.0 0.0 1.0)) (struct :`Pitch` 90.0 :`Yaw` 180.0) (`KismetMathLibrary.Conv_DoubleToVector` (/ _grid_tile_size_y (* (`.MaxValue` (`KismetMathLibrary.MaxOfIntArray` (`local.TextLenght`))) 30.0)))) false false)
              (else
                (`self.DestroyTextActor` (`local.Index`))))))
        (else
          (`self.DestroyTextActor` (`local.Index`) :!label _label)))
      (else
        (goto _label)))))

(fn `UserConstructionScript`)

(fn `WantToDisplayAnyText`
  (returns (ReturnValue :type Boolean))
  (return (or (`self.Show Tile Indexes`) (`self.ShowCostToEnterTile`) (`self.ShowMinCostToTarget`) (`self.ShowCostFromStart`) (`self.ShowSortOrder`))))