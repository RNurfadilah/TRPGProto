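; BP_WhiteMagicBase is the base actor for White Magic abilities, applying negated magic damage to its spell target as soon as it spawns.
; On BeginPlay it runs the parent logic, then asks the instigating BP_UnitBase's combat component for the base damage of this spell class.
; It sends that value times -1 through ApplyDamage with the configured damage type, so restorative effects reuse the damage pipeline.
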(event `self.ReceiveBeginPlay`
  (`parent.ReceiveBeginPlay`)
  (bind _asbp_unit_base (cast `/Game/Blueprints/Characters/Unit/BP_UnitBase` (`self.GetInstigator`)))
  (bind _returnvalue (`/Game/Blueprints/Characters/Unit/BP_CombatComponent.CalculateMagicBaseDamage` (`/Game/Blueprints/Characters/Unit/BP_UnitBase.BP_CombatComponent` _asbp_unit_base) (`GameplayStatics.GetObjectClass` self)))
  (`GameplayStatics.ApplyDamage` (`self.SpellTarget`) (* _returnvalue -1.0) null (`self.GetInstigator`) (`self.Damage Type Class`)))

(fn `UserConstructionScript`
  (`parent.UserConstructionScript`))