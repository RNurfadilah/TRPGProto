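; BP_Projectile is a unit ability projectile that deals damage when it hits and then destroys itself.
; At BeginPlay its sphere ignores the instigator while moving.
; On Hit it casts the instigator to BP_UnitBase, takes damage from that unit's combat component and applies it to the component's UnitTarget rather than the actor struck.
; The sphere overlap handler is empty, and the impact effect spawn is unconnected.
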(event `self.ReceiveBeginPlay`
  (`PrimitiveComponent.IgnoreActorWhenMoving` (`self.Sphere`) (`self.GetInstigator`) true))

(event `self.Sphere.OnComponentBeginOverlap`
  (params (OverlappedComponent :type "PrimitiveComponent Object Reference") (OtherActor :type "Actor Object Reference") (OtherComp :type "PrimitiveComponent Object Reference") (OtherBodyIndex :type Integer) (bFromSweep :type Boolean) (SweepResult :type "HitResult Structure (by ref)")))

(event `self.ReceiveHit`
  (params (MyComp :type "PrimitiveComponent Object Reference") (Other :type "Actor Object Reference") (OtherComp :type "PrimitiveComponent Object Reference") (bSelfMoved :type Boolean) (HitLocation :type "Vector Structure") (HitNormal :type "Vector Structure") (NormalImpulse :type "Vector Structure") (Hit :type "HitResult Structure (by ref)"))
  (bind _asbp_unit_base (cast `/Game/Blueprints/Characters/Unit/BP_UnitBase` (`self.GetInstigator`)))
  (bind _bp_combatcomponent (`/Game/Blueprints/Characters/Unit/BP_UnitBase.BP_CombatComponent` _asbp_unit_base))
  (bind _basedamage (`/Game/Blueprints/Characters/Unit/BP_CombatComponent.CalculateDamage` _bp_combatcomponent))
  (`GameplayStatics.ApplyDamage` (`/Game/Blueprints/Characters/Unit/BP_CombatComponent.UnitTarget` _bp_combatcomponent) _basedamage null _asbp_unit_base (`self.Damage Type Class`))
  (`self.K2_DestroyActor`))

(fn `UserConstructionScript`)