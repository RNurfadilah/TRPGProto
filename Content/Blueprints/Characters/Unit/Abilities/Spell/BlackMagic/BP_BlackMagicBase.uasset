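; BP_BlackMagicBase is the base Blueprint for black magic spell actors that damage a target.
; On BeginPlay it runs the parent logic, then casts its instigator to BP_UnitBase and gets base damage from that unit's combat component using the spell's own class.
; After a fixed short delay it applies that damage to SpellTarget with its damage type, crediting the instigator as damage causer.
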(event `self.ReceiveBeginPlay`
  (`parent.ReceiveBeginPlay`)
  (bind _asbp_unit_base (cast `/Game/Blueprints/Characters/Unit/BP_UnitBase` (`self.GetInstigator`)))
  (bind _returnvalue (`/Game/Blueprints/Characters/Unit/BP_CombatComponent.CalculateMagicBaseDamage` (`/Game/Blueprints/Characters/Unit/BP_UnitBase.BP_CombatComponent` _asbp_unit_base) (`GameplayStatics.GetObjectClass` self)))
  (`KismetSystemLibrary.Delay` 2.0)
  (`GameplayStatics.ApplyDamage` (`self.SpellTarget`) _returnvalue null (`self.GetInstigator`) (`self.Damage Type Class`)))

(fn `UserConstructionScript`
  (`parent.UserConstructionScript`))