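; Base unit character Blueprint that manages HP and MP pools for combat.
; On BeginPlay it derives max HP and MP from BPCombatComponent's base stats multiplied by its stat modifiers, then fills both.
; AnyDamage plays an optional hit-react montage, then subtracts the component's resistance-adjusted damage from clamped HP and debug-prints the result.
; SpendMP deducts a clamped cost and fires the MPSpent dispatcher; zero HP triggers no handling here.
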(event `self.ReceiveBeginPlay`
  (bind _bp_combatcomponent (`self.BP_CombatComponent`))
  (bind ((`HP_3_0241C320447E11AD7F3D9D8990B6F9FD` _hp) (`MP_15_FE6181714D2971CDA389A79C08F02B5B` _mp)) (break `/Game/Blueprints/Characters/Unit/Data/S_StatTable` (`/Game/Blueprints/Characters/Unit/BP_CombatComponent.BaseUnitStat` _bp_combatcomponent)))
  (bind ((`HP_19_0241C320447E11AD7F3D9D8990B6F9FD` _hp_2) (`MP_20_FE6181714D2971CDA389A79C08F02B5B` _mp_2)) (break `/Game/Blueprints/Characters/Unit/Data/S_StatModifier` (`/Game/Blueprints/Characters/Unit/BP_CombatComponent.UnitStatModifier` _bp_combatcomponent)))
  (bind _output_get (set `self.HP_Max` (* _hp _hp_2)))
  (set `self.HP_Current` _output_get)
  (bind _output_get_2 (set `self.MP_Max` (* _mp _mp_2)))
  (set `self.MP_Current` _output_get_2))

(event `self.ReceiveAnyDamage`
  (params (Damage :type "Float (single-precision)") (DamageType :type "DamageType Object Reference") (InstigatedBy :type "Controller Object Reference") (DamageCauser :type "Actor Object Reference"))
  (`|ExecutionSequence`
    (:`then_0`
      (bind _hitreactanimation (`self.HitReactAnimation`)
        (:`then`
          (`|PlayMontage` (`self.Mesh`) _hitreactanimation))
        (:`else`)))
    (:`then_1`
      (bind _newdamage (`/Game/Blueprints/Characters/Unit/BP_CombatComponent.CalculateDamageResistance` (`self.BP_CombatComponent`) Damage))
      (bind _output_get (set `self.HP_Current` (`KismetMathLibrary.FClamp` (- (`self.HP_Current`) _newdamage) 0.0 (`self.HP_Max`))))
      (`KismetSystemLibrary.PrintString` (`KismetStringLibrary.Conv_DoubleToString` _output_get)))))

(fn `SpendMP`
  (params (MPCost :type "Float (double-precision)"))
  (set `self.MP_Current` (`KismetMathLibrary.FClamp` (- (`self.MP_Current`) MPCost) 0.0 (`self.MP_Max`)))
  (`self.MPSpent`))

(fn `UserConstructionScript`)