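; Combat component on a grid-battle unit that runs its timed turns and performs melee, ranged and magic attacks on a chosen target.
; A Speed-based timer requests turns from GM_Core; player units get a battle HUD and target selection through BP_PC, while enemy units run AI.
; Attacks play montages, spawn projectiles or spells on notifies, then end the turn and restart the timer.
; It also calculates damage and resistance from data-table stats and modifiers.
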(event `self.ReceiveBeginPlay`
  (set `self.Speed` (`KismetMathLibrary.RandomFloatInRange` 0.0 10.0))
  (bind _asbp_unit_base (cast `/Game/Blueprints/Characters/Unit/BP_UnitBase` (`self.GetOwner`)))
  (bind _output_get (set `self.UnitCharacter` _asbp_unit_base))
  (set `self.BattlePosition` (`Actor.GetTransform` _output_get))
  (bind _asbp_pc (cast `/Game/Blueprints/Cores/Player/BP_PC` (`GameplayStatics.GetPlayerController` 0)))
  (set `self.Controller` _asbp_pc)
  (`self.BeginBattle`)
  (bind _returnvalue (`|GetDataTableRow` "/Game/Blueprints/Characters/Unit/Utilities/DT_BaseStat.DT_BaseStat" (`KismetStringLibrary.Conv_StringToName` (`KismetStringLibrary.Conv_IntToString` (`self.UnitLevel`))))
    (:`then`
      (set `self.BaseUnitStat` _returnvalue))))

(event `AttackCommand`
  (if (`self.IsRangedCharacter`)
    (`self.RangedAttack`)
    (else
      (`self.MeleeAttack`))))

(event `MeleeAttack`
  (bind _unitcharacter (`self.UnitCharacter`))
  (`Actor.K2_SetActorRotation` _unitcharacter (`KismetMathLibrary.FindLookAtRotation` (`Actor.K2_GetActorLocation` _unitcharacter) (`Actor.K2_GetActorLocation` (`self.UnitTarget`))) false)
  (`|ExecutionSequence`
    (:`then_0`
      (bind _unitbattlewindow (`self.UnitBattleWindow`)
        (:`then`
          (`Widget.RemoveFromParent` _unitbattlewindow))
        (:`else`)))
    (:`then_1`
      (`|PlayMontage` (`Character.Mesh` (`self.UnitCharacter`)) (`self.AttackMontage`)
        (:`OnCompleted`
          (`KismetSystemLibrary.Delay` 2.0)
          (`self.EndUnitTurn`))))))

(event `RangedAttack`
  (bind _unitcharacter (`self.UnitCharacter`))
  (bind _unitcharacter_2 (`self.UnitCharacter`))
  (`Actor.K2_SetActorRotation` _unitcharacter_2 (`KismetMathLibrary.FindLookAtRotation` (`Actor.K2_GetActorLocation` _unitcharacter_2) (`Actor.K2_GetActorLocation` (`self.UnitTarget`))) false)
  (`|ExecutionSequence`
    (:`then_0`
      (bind _unitbattlewindow (`self.UnitBattleWindow`)
        (:`then`
          (`Widget.RemoveFromParent` _unitbattlewindow))
        (:`else`)))
    (:`then_1`
      (`|PlayMontage` (`Character.Mesh` (`self.UnitCharacter`)) (`self.AttackMontage`)
        (:`OnCompleted`
          (`KismetSystemLibrary.Delay` 2.0)
          (`self.EndUnitTurn`))
        (:`OnNotifyBegin`
          (`|SpawnActorFromClass` (`self.ProjectileClass`) (`Actor.GetTransform` _unitcharacter) "Undefined" "OverrideRootScale" null _unitcharacter))))))

(event `MagicCommand`
  (params (Ability :type "/Game/Blueprints/Characters/Unit/Abilities/Spell/BP_MagicBase Class Reference"))
  (bind _unitcharacter (`self.UnitCharacter`))
  (`Actor.K2_SetActorRotation` _unitcharacter (`KismetMathLibrary.FindLookAtRotation` (`Actor.K2_GetActorLocation` _unitcharacter) (`Actor.K2_GetActorLocation` (`self.UnitTarget`))) false)
  (`|ExecutionSequence`
    (:`then_0`
      (bind _unitbattlewindow (`self.UnitBattleWindow`)
        (:`then`
          (`Widget.RemoveFromParent` _unitbattlewindow))
        (:`else`)))
    (:`then_1`
      (`|PlayMontage` (`Character.Mesh` (`self.UnitCharacter`)) (`self.MagicCastMontage`)
        (:`OnCompleted`
          (`KismetSystemLibrary.Delay` 2.0)
          (`self.EndUnitTurn`))
        (:`OnNotifyBegin`
          (`|SpawnActorFromClass` Ability (`self.GetSpellSpawnPosition` (`.SpawnType` (defaults `Object` Ability))) "Undefined" "OverrideRootScale" null (`self.UnitTarget`) (`self.UnitCharacter`)))))))

(fn `AttackSelectedTarget`
  (params (UnitTarget :type "/Game/Blueprints/Characters/Unit/BP_UnitBase Object Reference") (UnitIndex :type "IntPoint Structure"))
  (set `self.UnitTarget` UnitTarget)
  (bind _selectedability (`self.SelectedAbility`)
    (:`then`
      (`self.MagicCommand` _selectedability))
    (:`else`
      (`self.AttackCommand`))))

(fn `BeginBattle`
  (bind _returnvalue (`KismetSystemLibrary.K2_SetTimer` self "RequestTurn" (+ (* (- 1.0 (`KismetMathLibrary.NormalizeToRange` (`self.Speed`) 0.0 255.0)) (- (`self.MaxActionTime`) (`self.MinActionTime`))) (`self.MinActionTime`))))
  (set `self.ActionTimer` _returnvalue))

(fn `CalculateBaseDamage`
  (returns (CalculatedDamage :type "Float (double-precision)"))
  (return (* (* (* (`.STR_6_697B08DE4A5E008258E05BB79AED77DF` (break `/Game/Blueprints/Characters/Unit/Utilities/S_StatTable` (`self.BaseUnitStat`))) (`.STR_21_697B08DE4A5E008258E05BB79AED77DF` (break `/Game/Blueprints/Characters/Unit/Utilities/S_StatModifier` (`self.UnitStatModifier`)))) 5.0) (`KismetMathLibrary.RandomFloatInRange` 0.9 1.1))))

(fn `CalculateDamage`
  (returns (BaseDamage :type "Float (double-precision)"))
  (bind _calculateddamage (`self.CalculateBaseDamage`))
  (return _calculateddamage))

(fn `CalculateDamageResistance`
  (params (BaseDamage :type "Float (double-precision)"))
  (returns (NewDamage :type "Float (double-precision)"))
  (return (/ (`KismetMathLibrary.MultiplyMultiply_FloatFloat` BaseDamage 2.0) (+ BaseDamage (* (`.DEF_19_279B3F4C4F9F4A13C4B7F7ABFE64E83E` (break `/Game/Blueprints/Characters/Unit/Utilities/S_StatTable` (`self.BaseUnitStat`))) (`.DEF_26_279B3F4C4F9F4A13C4B7F7ABFE64E83E` (break `/Game/Blueprints/Characters/Unit/Utilities/S_StatModifier` (`self.UnitStatModifier`))))))))

(fn `CalculateMagicBaseDamage`
  (params (SpellClass :type "/Game/Blueprints/Characters/Unit/Abilities/Spell/BP_MagicBase Class Reference"))
  (returns (ReturnValue :type "Float (double-precision)"))
  (bind (_abilityname _rank _spelltarget _spellpowertable) (defaults `Object` (`local.SpellClass`)))
  (return (* (* (`.INT_20_88F971A44C654327A1B16090C406AD05` (break `/Game/Blueprints/Characters/Unit/Utilities/S_StatTable` (`self.BaseUnitStat`))) (`.INT_27_88F971A44C654327A1B16090C406AD05` (break `/Game/Blueprints/Characters/Unit/Utilities/S_StatModifier` (`self.UnitStatModifier`)))) (* (`KismetMathLibrary.Sqrt` (`BlueprintMapLibrary.Map_Find` _spellpowertable _rank)) 2.0))))

(fn `EndUnitTurn`
  (locals (StatesNeedToClear :type "Array of /Game/Blueprints/Cores/Utility/E_TileState Enum"))
  (bind _controller (`self.Controller`))
  (remove `/Game/Blueprints/Cores/Player/BP_PC.OnSelectedUnitAsTarget` (`self.Controller`) (`|CreateDelegate` :!event `AttackSelectedTarget`))
  (for _array_element (`local.StatesNeedToClear`)
    (`/Game/Blueprints/Cores/Grid/BP_Grid.ClearStateFromTiles` (`/Game/Blueprints/Characters/Unit/BP_UnitBase.Grid` (`self.UnitCharacter`)) _array_element))
  (set `/Game/Blueprints/Cores/Player/BP_PC.SelectedTile` (make `IntPoint` -999 -999) _controller)
  (set `/Game/Blueprints/Cores/Player/BP_PC.SelectedUnit` null _controller)
  (set `/Game/Blueprints/Cores/Player/BP_PC.IsSelectingTarget` false _controller)
  (set `self.SelectedAbility` null)
  (`self.TurnEnded`)
  (`self.BeginBattle`))

(fn `GetRangePosition`
  (params (TargettingEnemy :type Boolean :default true))
  (returns (ReturnValue :type "Vector Structure"))
  (bind _unitcharacter (`self.UnitCharacter`))
  (bind _returnvalue (`Actor.K2_GetActorLocation` (`self.UnitCharacter`)))
  (return (`KismetMathLibrary.SelectVector` (+ _returnvalue (* (`KismetMathLibrary.GetDirectionUnitVector` _returnvalue (`Actor.K2_GetActorLocation` (`self.UnitTarget`))) 500.0)) (+ (`Actor.K2_GetActorLocation` _unitcharacter) (* (`Actor.GetActorForwardVector` _unitcharacter) 500.0)) TargettingEnemy)))

(fn `GetSpellRange`
  (params (Ability :type "/Game/Blueprints/Characters/Unit/Abilities/Spell/BP_MagicBase Class Reference") (Index :type "IntPoint Structure") (`AI Unit` :type Boolean))
  (returns (RangeIndexes :type "Array of IntPoint Structure"))
  (bind _ability (`local.Ability`))
  (bind _selectedability (`self.SelectedAbility`))
  (bind (_rangepattern _rangeminmax) (break `/Game/Blueprints/Characters/Unit/Utilities/S_SpellData_Cast` (select `bool` (`KismetSystemLibrary.IsValidClass` _selectedability) :`false` (`self.AttackPattern`) :`true` (defaults `Object` _selectedability))))
  (`|ExecutionSequence`
    (:`then_0`
      (if (`KismetSystemLibrary.IsValidClass` _ability)
        (set `self.SelectedAbility` _ability)))
    (:`then_1`
      (bind _indexes (`/Game/Blueprints/Characters/Unit/Utilities/BFL_Spells.GetIndexesFromPatternAndRange` (select `bool` (`local.AI Unit`) :`false` (`/Game/Blueprints/Cores/Player/BP_PC.ActiveTile` (`self.Controller`)) :`true` (`local.Index`)) _rangepattern _rangeminmax))
      (return _indexes))))

(fn `GetSpellSpawnPosition`
  (params (SpawnType :type "/Game/Blueprints/Characters/Unit/Utilities/E_SpellSpawnType Enum" :default "NewEnumerator0"))
  (returns (SpawnTransform :type "Transform Structure"))
  (bind _unitcharacter (`self.UnitCharacter`))
  (bind _unittarget (`self.UnitTarget`))
  (bind (_returnvalue_location _returnvalue_rotation _returnvalue_scale) (`KismetMathLibrary.BreakTransform` (`Actor.GetTransform` _unitcharacter)))
  (bind (_returnvalue_location_2 _returnvalue_rotation_2 _returnvalue_scale_2) (`KismetMathLibrary.BreakTransform` (`Actor.GetTransform` _unittarget)))
  (return (select `/Game/Blueprints/Characters/Unit/Utilities/E_SpellSpawnType` SpawnType :`NewEnumerator0` (`KismetMathLibrary.MakeTransform` (+ _returnvalue_location (* (`Actor.GetActorForwardVector` _unitcharacter) 50.0)) _returnvalue_rotation _returnvalue_scale) :`NewEnumerator1` (`KismetMathLibrary.MakeTransform` (+ _returnvalue_location_2 (* (`Actor.GetActorUpVector` _unittarget) 200.0)) _returnvalue_rotation_2 _returnvalue_scale_2) :`NewEnumerator2` (`Actor.GetTransform` _unittarget))))

(fn `RequestTurn`
  (bind _asgm_core (cast `/Game/Blueprints/Cores/GM_Core` (`GameplayStatics.GetGameMode`)))
  (`/Game/Blueprints/Cores/GM_Core.TurnRequest` _asgm_core (`self.UnitCharacter`)))

(fn `SelectAttackTarget`
  (params (Ability :type "/Game/Blueprints/Characters/Unit/Abilities/Spell/BP_MagicBase Class Reference"))
  (bind _controller (`self.Controller`))
  (`|ExecutionSequence`
    (:`then_0`
      (if (`KismetSystemLibrary.IsValidClass` (`local.Ability`))
        (bind _output_get (set `self.SelectedAbility` (`local.Ability`)))
        (set `self.IsTargettingEnemy` (`KismetMathLibrary.ClassIsChildOf` _output_get "/Game/Blueprints/Characters/Unit/Abilities/Spell/BlackMagic/BP_BlackMagicBase.BP_BlackMagicBase_C"))
        (else
          (set `self.IsTargettingEnemy` true))))
    (:`then_1`
      (`/Game/Blueprints/Cores/Player/BP_PC.ShowAttackPattern` _controller)
      (set `/Game/Blueprints/Cores/Player/BP_PC.IsSelectingTarget` true _controller)
      (add `/Game/Blueprints/Cores/Player/BP_PC.OnSelectedUnitAsTarget` _controller (`|CreateDelegate` :!event `AttackSelectedTarget`)))))

(fn `SetCamera`
  (bind _returnvalue (`GameplayStatics.GetActorOfClass` "/Game/Blueprints/Characters/BP_DynamicCamera.BP_DynamicCamera_C"))
  (`PlayerController.SetViewTargetWithBlend` (`GameplayStatics.GetPlayerController` 0) _returnvalue 0.0 "VTBlend_Linear" 0.0 false)
  (message `/Game/Blueprints/Characters/BPI_DynamicCamera.SetDynamicLocation` _returnvalue (`self.UnitCharacter`) (0.0 0.0 0.0)))

(fn `StartUnitTurn`
  (bind _unitbattlewindow (`self.UnitBattleWindow`))
  (if (`KismetMathLibrary.ClassIsChildOf` (`GameplayStatics.GetObjectClass` (`self.UnitCharacter`)) "/Game/Blueprints/Characters/Unit/Characters/BP_PlayerUnitBase.BP_PlayerUnitBase_C")
    (bind _returnvalue (`|CreateWidget` "/Game/UIs/CombatWidget/WBP_UnitBattleHUD.WBP_UnitBattleHUD_C" null (`self.UnitCharacter`)))
    (bind _output_get (set `self.UnitBattleWindow` _returnvalue))
    (`UserWidget.AddToViewport` _output_get 0)
    (`/Game/Blueprints/Cores/Player/BP_PC.OnPlayerUnitActive` (`self.Controller`))
    (add `/Game/UIs/CombatWidget/WBP_ActionCommand.CommandAttack` (`/Game/UIs/CombatWidget/WBP_UnitBattleHUD.WBP_ActionCommand` _unitbattlewindow) (`|CreateDelegate` :!event `SelectAttackTarget`))
    (add `/Game/UIs/CombatWidget/WBP_MagicWindow.AbilityChosenTarget` (`/Game/UIs/CombatWidget/WBP_UnitBattleHUD.WBP_MagicWindow` _unitbattlewindow) (`|CreateDelegate` :!event `SelectAttackTarget`))
    (else
      (bind _asbp_enemy_unit_base (cast `/Game/Blueprints/Characters/Unit/Enemies/BP_EnemyUnitBase` (`self.UnitCharacter`)))
      (`/Game/Blueprints/Characters/Unit/Enemies/BP_EnemyUnitBase.AIPlayTurn` _asbp_enemy_unit_base))))