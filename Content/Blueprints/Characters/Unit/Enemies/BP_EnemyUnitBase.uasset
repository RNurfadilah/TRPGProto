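; Base enemy unit for grid-based tactical combat, running its turn AI as an asynchronous chain of delayed states and pathfinding callbacks.
; It scores basic attacks and affordable black or white magic from every reachable tile by damage, target HP, mana cost and travel distance.
; It walks to the best option and acts through the combat component.
; Without one, it moves toward or away from enemies or allies per MovementLogic, then ends its turn.
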(event `EventRunAILogic`
  (`self.SetAIStateWithDelay` "NewEnumerator1")
  (`self.DecideWhichSpellToCast`))

(event `DecideWhichSpellToCast`
  (bind _gridpathfinding_ai (`/Game/Blueprints/Cores/Grid/BP_Grid.GridPathFinding_AI` (`self.Grid`)))
  (`self.SetAIStateWithDelay` "NewEnumerator2")
  (set `self.AISpellCasting` (struct))
  (add `/Game/Blueprints/Cores/Grid/BP_GridPathFinding.OnPathFindingCompleted` _gridpathfinding_ai (delegate `OnCompletedSpellReachables`))
  (`/Game/Blueprints/Cores/Grid/BP_GridPathFinding.Find Path` _gridpathfinding_ai (`self.Index`) (make `IntPoint` -999 -999) (`self.CanMoveDiagonally`) 0.1 15.0 true (`self.PathCurrent`)))

(event `OnCompletedSpellReachables`
  (params (Path :type "Array of IntPoint Structure (by ref)"))
  (remove `/Game/Blueprints/Cores/Grid/BP_GridPathFinding.OnPathFindingCompleted` (`/Game/Blueprints/Cores/Grid/BP_Grid.GridPathFinding_AI` (`self.Grid`)) (delegate `OnCompletedSpellReachables`))
  (bind _spells (`self.GetCastableSpells`))
  (for _array_element _spells
    (for _array_element_2 Path
      (`self.CalculateSpellScoreAndUpdateSpellCasting` (struct) _array_element_2 _array_element)))
  (`|ExecutionSequence`
    (:`then_0`
      (for _array_element_3 Path
        (`self.CalculateSpellScoreAndUpdateSpellCasting` (struct) _array_element_3)))
    (:`then_1`
      (`self.DecideWhichSpellToCast_Done`))))

(event `DecideWhichSpellToCast_Done`
  (if (`.IsSpellValid_1_CB98530F4E454A2EEF2DC8A3B783A42B` (break `/Game/Blueprints/Characters/Unit/Enemies/AI/S_UnitAISpellCastingData` (`self.AISpellCasting`)))
    (`self.MoveToSpellCastingLocation`)
    (else
      (`self.DecideWhereToEndTurn`))))

(event `MoveToSpellCastingLocation`
  (bind _gridpathfinding_ai (`/Game/Blueprints/Cores/Grid/BP_Grid.GridPathFinding_AI` (`self.Grid`)))
  (if (!= (`self.Index`) (`.OriginalIndex_7_81BAF91E43F5677390664B971A92EFA7` (break `/Game/Blueprints/Characters/Unit/Enemies/AI/S_UnitAISpellCastingData` (`self.AISpellCasting`))))
    (`self.SetAIStateWithDelay` "NewEnumerator3")
    (add `/Game/Blueprints/Cores/Grid/BP_GridPathFinding.OnPathFindingCompleted` _gridpathfinding_ai (delegate `OnCompletedSpellPath`))
    (`/Game/Blueprints/Cores/Grid/BP_GridPathFinding.Find Path` _gridpathfinding_ai (`self.Index`) (`.OriginalIndex_7_81BAF91E43F5677390664B971A92EFA7` (break `/Game/Blueprints/Characters/Unit/Enemies/AI/S_UnitAISpellCastingData` (`self.AISpellCasting`))) (`self.CanMoveDiagonally`) 0.1 15.0 false (`self.PathCurrent`))
    (else
      (`self.MoveToSpellCastingLocation_Done`))))

(event `OnCompletedSpellPath`
  (params (Path :type "Array of IntPoint Structure (by ref)"))
  (remove `/Game/Blueprints/Cores/Grid/BP_GridPathFinding.OnPathFindingCompleted` (`/Game/Blueprints/Cores/Grid/BP_Grid.GridPathFinding_AI` (`self.Grid`)) (delegate `OnCompletedSpellPath`))
  (add `self.OnUnitFinishedWalking` (delegate `OnCompletedSpellUnitWalking`))
  (`self.MoveToPath` Path))

(event `OnCompletedSpellUnitWalking` :!signature `self.OnUnitFinishedWalking`
  (params (Unit :type "/Game/Blueprints/Characters/Unit/BP_UnitBase Object Reference"))
  (remove `self.OnUnitFinishedWalking` (delegate `OnCompletedSpellUnitWalking`))
  (`self.MoveToSpellCastingLocation_Done`))

(event `MoveToSpellCastingLocation_Done`
  (`self.CastSpell`))

(event `CastSpell`
  (bind _bp_combatcomponent (`self.BP_CombatComponent`))
  (bind ((`Spell_13_037AD59C41FE6283484473AC2304B145` _spell) (`TargetUnit_16_4E6D7BD749C7F36BCCBE3196BF21F1EF` _targetunit)) (break `/Game/Blueprints/Characters/Unit/Enemies/AI/S_UnitAISpellCastingData` (`self.AISpellCasting`)))
  (`self.SetAIStateWithDelay` "NewEnumerator4")
  (set `/Game/Blueprints/Characters/Unit/BP_CombatComponent.UnitTarget` _targetunit (`self.BP_CombatComponent`))
  (if (`KismetSystemLibrary.IsValidClass` _spell)
    (`/Game/Blueprints/Characters/Unit/BP_CombatComponent.MagicCommand` _bp_combatcomponent _spell)
    (else
      (`/Game/Blueprints/Characters/Unit/BP_CombatComponent.AttackCommand` _bp_combatcomponent)))
  (`self.CastSpell_Done`))

(event `CastSpell_Done`
  (`self.SetAIStateWithDelay` "NewEnumerator7"))

(event `DecideWhereToEndTurn`
  (bind _gridpathfinding_ai (`/Game/Blueprints/Cores/Grid/BP_Grid.GridPathFinding_AI` (`self.Grid`)))
  (`self.SetAIStateWithDelay` "NewEnumerator5")
  (if (> (`self.PathCurrent`) 0)
    (add `/Game/Blueprints/Cores/Grid/BP_GridPathFinding.OnPathFindingCompleted` _gridpathfinding_ai (delegate `OnCompletedEndTurnReachables`))
    (`/Game/Blueprints/Cores/Grid/BP_GridPathFinding.Find Path` _gridpathfinding_ai (`self.Index`) (make `IntPoint` -999 -999) false 0.1 15.0 true (`self.PathCurrent`))
    (else
      (`self.DecideWhereToEndTurn_Done` (`|MakeArray` (struct) :!type "IntPoint Structure")))))

(event `OnCompletedEndTurnReachables`
  (params (Path :type "Array of IntPoint Structure (by ref)"))
  (bind _gridpathfinding_ai (`/Game/Blueprints/Cores/Grid/BP_Grid.GridPathFinding_AI` (`self.Grid`)))
  (remove `/Game/Blueprints/Cores/Grid/BP_GridPathFinding.OnPathFindingCompleted` _gridpathfinding_ai (delegate `OnCompletedEndTurnReachables`))
  (bind _index (`self.FindBestIndexInReachables` Path))
  (add `/Game/Blueprints/Cores/Grid/BP_GridPathFinding.OnPathFindingCompleted` _gridpathfinding_ai (delegate `OnCompletedEndTurnPath`))
  (`/Game/Blueprints/Cores/Grid/BP_GridPathFinding.Find Path` _gridpathfinding_ai (`self.Index`) _index false 0.1 15.0 false (`self.PathCurrent`)))

(event `OnCompletedEndTurnPath`
  (params (Path :type "Array of IntPoint Structure (by ref)"))
  (remove `/Game/Blueprints/Cores/Grid/BP_GridPathFinding.OnPathFindingCompleted` (`/Game/Blueprints/Cores/Grid/BP_Grid.GridPathFinding_AI` (`self.Grid`)) (delegate `OnCompletedEndTurnPath`))
  (`self.DecideWhereToEndTurn_Done` Path))

(event `DecideWhereToEndTurn_Done`
  (params (Path :type "Array of IntPoint Structure"))
  (`self.MoveToEndTurnLocation` Path))

(event `MoveToEndTurnLocation`
  (params (Path :type "Array of IntPoint Structure"))
  (if (> (`KismetArrayLibrary.Array_Length` Path) 0)
    (`self.SetAIStateWithDelay` "NewEnumerator6")
    (add `self.OnUnitFinishedWalking` (delegate `OnCompletedEndTurnUnitWalking`))
    (`self.MoveToPath` Path)
    (else
      (`self.MoveToEndTurnLocation_Done`))))

(event `OnCompletedEndTurnUnitWalking` :!signature `self.OnUnitFinishedWalking`
  (params (Unit :type "/Game/Blueprints/Characters/Unit/BP_UnitBase Object Reference"))
  (remove `self.OnUnitFinishedWalking` (delegate `OnCompletedEndTurnUnitWalking`))
  (`self.MoveToEndTurnLocation_Done`))

(event `MoveToEndTurnLocation_Done`
  (`self.SetAIStateWithDelay` "NewEnumerator7")
  (`self.AIEndTurn`))

(fn `AIEndTurn`
  (`/Game/Blueprints/Characters/Unit/BP_CombatComponent.EndUnitTurn` (`self.BP_CombatComponent`)))

(fn `AIPlayTurn`
  (`self.EventRunAILogic`))

(fn `CalculateImpactScore`
  (params (Spell :type "/Game/Blueprints/Characters/Unit/Abilities/Spell/BP_MagicBase Class Reference") (AttackedUnit :type "/Game/Blueprints/Characters/Unit/BP_UnitBase Object Reference"))
  (returns (ImpactScore :type "Float (double-precision)"))
  (locals (HpValue :type "Float (double-precision)") (MpValue :type "Float (double-precision)") (KillingValue :type "Float (double-precision)") (Cost :type "Float (double-precision)") (DamageValue :type "Float (double-precision)") (HpScore :type "Float (double-precision)") (DamageScore :type "Float (double-precision)") (CalculatedDamage :type "Float (double-precision)") (HpModifier :type "Float (double-precision)"))
  (bind _spell (`local.Spell`))
  (bind _attackedunit (`local.AttackedUnit`))
  (bind (_rank _manacosttable) (defaults `Object` (`local.Spell`)))
  (bind _returnvalue (* (`local.CalculatedDamage`) (`local.DamageValue`)))
  (set `local.HpValue` -1.0)
  (set `local.DamageValue` 10.0)
  (set `local.MpValue` 3.0)
  (set `local.KillingValue` 100.0)
  (set `local.HpModifier` 0.0)
  (`|ExecutionSequence`
    (:`then_0`
      (if (`KismetSystemLibrary.IsValidClass` (`local.Spell`))
        (set `local.Cost` (* (`BlueprintMapLibrary.Map_Find` _manacosttable _rank) (`local.MpValue`)))
        (set `local.HpModifier` (`KismetMathLibrary.SelectFloat` -500.0 0.0 (and (`KismetMathLibrary.ClassIsChildOf` (`local.Spell`) "/Game/Blueprints/Characters/Unit/Abilities/Spell/WhiteMagic/BP_WhiteMagicBase.BP_WhiteMagicBase_C") (== (`/Game/Blueprints/Characters/Unit/BP_UnitBase.HPCurrent` _attackedunit) (`/Game/Blueprints/Characters/Unit/BP_UnitBase.HPMax` _attackedunit)))))))
    (:`then_1`
      (set `local.HpScore` (* (`/Game/Blueprints/Characters/Unit/BP_UnitBase.HPCurrent` (`local.AttackedUnit`)) (`local.HpValue`)))
      (if (`KismetSystemLibrary.IsValidClass` (`local.Spell`))
        (bind _returnvalue_2 (`/Game/Blueprints/Characters/Unit/BP_CombatComponent.CalculateMagicBaseDamage` (`self.BP_CombatComponent`) _spell))
        (set `local.CalculatedDamage` _returnvalue_2)
        (if (`KismetMathLibrary.ClassIsChildOf` _spell "/Game/Blueprints/Characters/Unit/Abilities/Spell/BlackMagic/BP_BlackMagicBase.BP_BlackMagicBase_C")
          (bind _newdamage (`/Game/Blueprints/Characters/Unit/BP_CombatComponent.CalculateDamageResistance` (`/Game/Blueprints/Characters/Unit/BP_UnitBase.BP_CombatComponent` (`local.AttackedUnit`)) (`local.CalculatedDamage`)))
          (bind _output_get (set `local.CalculatedDamage` _newdamage))
          (if (<= (- (`/Game/Blueprints/Characters/Unit/BP_UnitBase.HPCurrent` (`local.AttackedUnit`)) _output_get) 0.0)
            (set `local.DamageScore` (+ _returnvalue 200.0))
            (else
              (set `local.DamageScore` _returnvalue)))
          (else
            (set `local.DamageScore` (* (`local.DamageValue`) (`local.CalculatedDamage`)))))
        (else
          (bind _calculateddamage (`/Game/Blueprints/Characters/Unit/BP_CombatComponent.CalculateBaseDamage` (`self.BP_CombatComponent`)))
          (bind _newdamage_2 (`/Game/Blueprints/Characters/Unit/BP_CombatComponent.CalculateDamageResistance` (`/Game/Blueprints/Characters/Unit/BP_UnitBase.BP_CombatComponent` (`local.AttackedUnit`)) _calculateddamage))
          (set `local.DamageScore` (* _newdamage_2 (`local.DamageValue`))))))
    (:`then_2`
      (return (+ (/ (+ (`local.HpScore`) (`local.DamageScore`)) (`KismetMathLibrary.FMax` (`local.Cost`) 1.0)) (`local.HpModifier`))))))

(fn `CalculateSpellScoreAndUpdateSpellCasting`
  (params (Target :type "IntPoint Structure") (Origin :type "IntPoint Structure") (Spell :type "/Game/Blueprints/Characters/Unit/Abilities/Spell/BP_MagicBase Class Reference"))
  (locals (AllUnitsExceptSelf :type "Map of IntPoint Structure to /Game/Blueprints/Characters/Unit/BP_UnitBase Object Reference") (AttackedIndexes :type "Array of IntPoint Structure") (TotalSpellScore :type "Float (double-precision)") (AttackedIndex :type "IntPoint Structure") (AttackedUnit :type "/Game/Blueprints/Characters/Unit/BP_UnitBase Object Reference") (AllAttackedUnits :type "Map of IntPoint Structure to /Game/Blueprints/Characters/Unit/BP_UnitBase Object Reference") (ImpactScore :type "Float (double-precision)") (IsWhiteMagic :type Boolean :default false))
  (`|ExecutionSequence`
    (:`then_0`
      (bind _output_get (set `local.IsWhiteMagic` (and (`KismetMathLibrary.ClassIsChildOf` (`local.Spell`) "/Game/Blueprints/Characters/Unit/Abilities/Spell/WhiteMagic/BP_WhiteMagicBase.BP_WhiteMagicBase_C") (`KismetSystemLibrary.IsValidClass` (`local.Spell`)))))
      (if _output_get
        (bind _units (`self.GetAllyUnits` false))
        (set `local.AllAttackedUnits` _units)
        (else
          (bind _units_2 (`self.GetEnemyUnits`))
          (set `local.AllAttackedUnits` _units_2))))
    (:`then_1`
      (bind _rangeindexes (`/Game/Blueprints/Characters/Unit/BP_CombatComponent.GetSpellRange` (`self.BP_CombatComponent`) (`local.Spell`) (`local.Origin`) true))
      (set `local.AttackedIndexes` _rangeindexes)
      (set `local.AttackedUnit` null)
      (set `local.TotalSpellScore` (* (`KismetMathLibrary.Distance2D` (`KismetMathLibrary.Conv_IntPointToVector2D` (`self.Index`)) (`KismetMathLibrary.Conv_IntPointToVector2D` (`local.Origin`))) -5.0))
      (for _array_element (`local.AttackedIndexes`)
        (bind _output_get_2 (set `local.AttackedIndex` _array_element))
        (if (`KismetMathLibrary.Equal_IntPointIntPoint` _output_get_2 (`self.Index`))
          (if (`local.IsWhiteMagic`)
            (set `local.AttackedUnit` self)
            (`/Engine/EditorBlueprintResources/StandardMacros.IsValid` (`local.AttackedUnit`) :!label _label
              (:`Is Valid`
                (bind _impactscore (`self.CalculateImpactScore` (`local.Spell`) (`local.AttackedUnit`)))
                (bind _output_get_3 (set `local.TotalSpellScore` (+ _impactscore (`local.TotalSpellScore`))))
                (if (> _output_get_3 (`.SpellScore_12_7E392FF54D22E45386B9179DAC9C6B73` (break `/Game/Blueprints/Characters/Unit/Enemies/AI/S_UnitAISpellCastingData` (`self.AISpellCasting`))))
                  (set `self.AISpellCasting` (make `/Game/Blueprints/Characters/Unit/Enemies/AI/S_UnitAISpellCastingData` true (`local.Spell`) (`local.Origin`) (`local.Target`) (`local.AttackedUnit`) (`local.TotalSpellScore`)))))))
          (else
            (set `local.AttackedUnit` (`BlueprintMapLibrary.Map_Find` (`local.AllAttackedUnits`) (`local.AttackedIndex`)))
            (goto _label)))))))

(fn `FindBestIndexInReachables`
  (params (Reachables :type "Array of IntPoint Structure (by ref)"))
  (returns (Index :type "IntPoint Structure"))
  (locals (EnemiesOrAllies :type "Array of IntPoint Structure"))
  (bind _movementlogic (`self.MovementLogic`))
  ;[0 0 0 1 14] 1. Find either enemies or allies on grid
  ; 2. Either move towards or away from the units found in 1
  (`|ExecutionSequence`
    (:`then_0`
      (switch `/Game/Blueprints/Characters/Unit/Enemies/AI/E_UnitAIMovementLogic` _movementlogic
        (:`NewEnumerator0`
          (bind _units (`self.GetEnemyUnits` :!label _label))
          (bind _keys (`BlueprintMapLibrary.Map_Keys` _units))
          (set `local.EnemiesOrAllies` _keys))
        (:`NewEnumerator1`
          (bind _units_2 (`self.GetAllyUnits` false :!label _label_2))
          (bind _keys_2 (`BlueprintMapLibrary.Map_Keys` _units_2))
          (set `local.EnemiesOrAllies` _keys_2))
        (:`NewEnumerator2`
          (goto _label))
        (:`NewEnumerator3`
          (goto _label_2))))
    (:`then_1`
      (switch `/Game/Blueprints/Characters/Unit/Enemies/AI/E_UnitAIMovementLogic` _movementlogic
        (:`NewEnumerator0`
          _)
        (:`NewEnumerator1`
          _)
        (:`NewEnumerator2`
          (bind _index (`self.FindFarthestIndex` (`local.Reachables`) (`local.EnemiesOrAllies`) :!label _label_3))
          (return _index))
        (:`NewEnumerator3`
          (goto _label_3)))
      (bind _index_2 (`self.FindClosestIndex` (`local.Reachables`) (`local.EnemiesOrAllies`)))
      (return _index_2))))

(fn `FindClosestIndex`
  (params (Reachables :type "Array of IntPoint Structure") (PossibleTarget :type "Array of IntPoint Structure"))
  (returns (Index :type "IntPoint Structure"))
  (locals (Ret :type "IntPoint Structure") (SmallestDistance :type Integer) (Reachable :type "IntPoint Structure") (Target :type "IntPoint Structure") (NewDistance :type Integer :default 0))
  (set `local.SmallestDistance` 999999)
  (for _array_element (`local.Reachables`)
    (set `local.Reachable` _array_element)
    (for _array_element_2 (`local.PossibleTarget`)
      (set `local.Target` _array_element_2)
      (bind _output_get (set `local.NewDistance` (`/Game/Blueprints/Cores/Grid/BP_GridPathFinding.GetMinimunCostBetweenTwoTiles` (`/Game/Blueprints/Cores/Grid/BP_Grid.GridPathFinding_AI` (`self.Grid`)) (`local.Reachable`) (`local.Target`) (`self.CanMoveDiagonally`))))
      (if (< _output_get (`local.SmallestDistance`))
        (set `local.Ret` (`local.Reachable`))
        (set `local.SmallestDistance` (`local.NewDistance`)))))
  (return (`local.Ret`)))

(fn `FindFarthestIndex`
  (params (Reachables :type "Array of IntPoint Structure") (IndexesToAvoid :type "Array of IntPoint Structure"))
  (returns (Index :type "IntPoint Structure"))
  (locals (Ret :type "IntPoint Structure") (BiggestDistance :type Integer) (Reachable :type "IntPoint Structure") (NewDistance :type Integer) (IndexToAvoid :type "IntPoint Structure"))
  (set `local.BiggestDistance` -999999)
  (for _array_element (`local.Reachables`)
    (set `local.Reachable` _array_element)
    (set `local.NewDistance` 999999999)
    (for _array_element_2 (`local.IndexesToAvoid`)
      (set `local.IndexToAvoid` _array_element_2)
      (set `local.NewDistance` (`KismetMathLibrary.Min` (`local.NewDistance`) (`/Game/Blueprints/Cores/Grid/BP_GridPathFinding.GetMinimunCostBetweenTwoTiles` (`/Game/Blueprints/Cores/Grid/BP_Grid.GridPathFinding_AI` (`self.Grid`)) (`local.Reachable`) (`local.IndexToAvoid`) (`self.CanMoveDiagonally`)))))
    (if (> (`local.NewDistance`) (`local.BiggestDistance`))
      (set `local.Ret` (`local.Reachable`))
      (set `local.BiggestDistance` (`local.NewDistance`))))
  (return (`local.Ret`)))

(fn `Get All Units`
  (params (IncludeSelf :type Boolean))
  (returns (AllUnits :type "Map of IntPoint Structure to /Game/Blueprints/Characters/Unit/BP_UnitBase Object Reference"))
  (locals (Ret :type "Map of IntPoint Structure to /Game/Blueprints/Characters/Unit/BP_UnitBase Object Reference") (U :type "/Game/Blueprints/Characters/Unit/BP_UnitBase Object Reference"))
  (bind _u (`local.U`))
  (bind _outactors (`GameplayStatics.GetAllActorsOfClass` "/Game/Blueprints/Characters/Unit/BP_UnitBase.BP_UnitBase_C"))
  (for _array_element _outactors
    (bind _output_get (set `local.U` _array_element))
    (if (or (!= _output_get self) (`local.IncludeSelf`))
      (`BlueprintMapLibrary.Map_Add` (`local.Ret`) (`/Game/Blueprints/Characters/Unit/BP_UnitBase.Index` _u) _u)))
  (return (`local.Ret`)))

(fn `GetAllyUnits`
  (params (IncludeSelf :type Boolean))
  (returns (Units :type "Map of IntPoint Structure to /Game/Blueprints/Characters/Unit/BP_UnitBase Object Reference"))
  (locals (Ret :type "Map of IntPoint Structure to /Game/Blueprints/Characters/Unit/BP_UnitBase Object Reference") (U :type "/Game/Blueprints/Characters/Unit/Enemies/BP_EnemyUnitBase Object Reference"))
  (bind _u (`local.U`))
  (bind _outactors (`GameplayStatics.GetAllActorsOfClass` "BP_EnemyUnitBase_C"))
  (for _array_element _outactors
    (bind _output_get (set `local.U` _array_element))
    (if (or (!= _output_get self) (`local.IncludeSelf`))
      (`BlueprintMapLibrary.Map_Add` (`local.Ret`) (`/Game/Blueprints/Characters/Unit/BP_UnitBase.Index` _u) _u)))
  (return (`local.Ret`)))

(fn `GetCastableSpells`
  (returns (Spells :type "Array of /Game/Blueprints/Characters/Unit/Abilities/Spell/BP_MagicBase Class Reference"))
  (locals (Ret :type "Array of /Game/Blueprints/Characters/Unit/Abilities/Spell/BP_MagicBase Class Reference"))
  (bind _bp_combatcomponent (`self.BP_CombatComponent`))
  (for _array_element (`/Game/Blueprints/Characters/Unit/BP_CombatComponent.BlackMagicAbilities` _bp_combatcomponent)
    (bind (_rank _manacosttable) (defaults `Object` _array_element))
    (if (< (`BlueprintMapLibrary.Map_Find` _manacosttable _rank) (`self.MPCurrent`))
      (`KismetArrayLibrary.Array_Add` (`local.Ret`) _array_element)))
  (for _array_element_2 (`/Game/Blueprints/Characters/Unit/BP_CombatComponent.WhiteMagicAbilities` _bp_combatcomponent)
    (bind (_rank_2 _manacosttable_2) (defaults `Object` _array_element_2))
    (if (< (`BlueprintMapLibrary.Map_Find` _manacosttable_2 _rank_2) (`self.MPCurrent`))
      (`KismetArrayLibrary.Array_Add` (`local.Ret`) _array_element_2)))
  (return (`local.Ret`)))

(fn `GetEnemyUnits`
  (returns (Units :type "Map of IntPoint Structure to /Game/Blueprints/Characters/Unit/BP_UnitBase Object Reference"))
  (locals (Ret :type "Map of IntPoint Structure to /Game/Blueprints/Characters/Unit/BP_UnitBase Object Reference"))
  (bind _outactors (`GameplayStatics.GetAllActorsOfClass` "/Game/Blueprints/Characters/Unit/Characters/BP_PlayerUnitBase.BP_PlayerUnitBase_C"))
  (for _array_element _outactors
    (`BlueprintMapLibrary.Map_Add` (`local.Ret`) (`/Game/Blueprints/Characters/Unit/BP_UnitBase.Index` _array_element) _array_element))
  (return (`local.Ret`)))

(fn `UserConstructionScript`
  (`parent.UserConstructionScript`))