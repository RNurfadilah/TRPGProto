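; BP_Unit is a character unit with click-to-move control, whose appearance is set by its UnitType.
; The construction script looks up default data for that type and applies its skeletal mesh and Anim Blueprint.
; Right mouse press traces under the cursor, picks running or walking speed by distance to the hit point, then calls SimpleMoveToLocation on player controller 0.
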(event `Key|RightMouseButton`
  (params (Key :type "Key Structure"))
  (:`Pressed`
    (`self.MoveToPoint`)))

(fn `GetDestinationToMove`
  (returns (Destination :type "Vector Structure"))
  (return (`.Location` (`GameplayStatics.BreakHitResult` (`PlayerController.GetHitResultUnderCursorByChannel` (`GameplayStatics.GetPlayerController` 0) "TraceTypeQuery1" true)))))

(fn `MoveToPoint`
  (locals (MoveDestination :type "Vector Structure"))
  (bind _charactermovement (`self.CharacterMovement`))
  (bind _destination (`self.GetDestinationToMove`))
  (bind _output_get (set `local.MoveDestination` _destination))
  (if (> (`KismetMathLibrary.VSize` (- _output_get (`self.K2_GetActorLocation`))) 150.0)
    (set `CharacterMovementComponent.MaxWalkSpeed` 600.0 _charactermovement)
    (else
      (set `CharacterMovementComponent.MaxWalkSpeed` 150.0 _charactermovement)))
  (`AIBlueprintHelperLibrary.SimpleMoveToLocation` (`GameplayStatics.GetPlayerController` 0) (`local.MoveDestination`)))

(fn `UserConstructionScript`
  (bind _mesh (`self.Mesh`))
  (bind _unitdata (`/Game/Blueprints/Characters/Utilities/BFL_Units.GetDefaultUnitDataFromUnitType` (`self.UnitType`)))
  (bind (_mesh_2 _animbp) (break `/Game/Blueprints/Characters/Utilities/S_UnitData_Assets` (`.Assets_5_D620F7834CFA35E3E90CEBBDD7D528B0` (break `/Game/Blueprints/Characters/Utilities/S_UnitData` _unitdata))))
  (`SkeletalMeshComponent.SetSkeletalMeshAsset` _mesh _mesh_2)
  (`SkeletalMeshComponent.SetAnimInstanceClass` _mesh _animbp))