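; Test game mode that runs a turn-based battle between party and enemy units.
; On BeginPlay it repositions the player pawn, gathers both sides and adds party units to the battle HUD.
; Turn requests fill a unique FIFO queue, with a DoOnce gate allowing one active turn and a turn-ended binding for handoff.
; Uncalled helper functions randomize unit speeds and spawn units at battle positions.
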(event `self.ReceiveBeginPlay`
  (`self.K2_SetActorLocation` (`GameplayStatics.GetPlayerPawn` 0) (-1160.0 -360.0 0.0) false false)
  (bind _outactors (`GameplayStatics.GetAllActorsOfClass` "/Game/Blueprints/Characters/Unit/BP_PlayerUnitBase.BP_PlayerUnitBase_C"))
  (set `self.PartyUnits` _outactors)
  (bind _outactors_2 (`GameplayStatics.GetAllActorsOfClass` "/Game/Blueprints/Characters/Unit/BP_EnemyUnitBase.BP_EnemyUnitBase_C"))
  (set `self.EnemyUnits` _outactors_2)
  (`KismetSystemLibrary.Delay` 0.2)
  (bind _asbp_pc (cast `/Game/Blueprints/Cores/BP_PC` (`GameplayStatics.GetPlayerController` 0)))
  (bind _output_get (set `self.Battle HUD` (`/Game/Blueprints/Cores/BP_PC.BattleHUD` _asbp_pc)))
  (for _array_element (`self.PartyUnits`)
    (`/Game/UIs/CombatWidget/WBP_BattleHUD.AddPartyUnitToHUD` _output_get _array_element)))

(event `TurnRequest`
  (params (Unit :type "/Game/Blueprints/Characters/Unit/BP_UnitBase Object Reference"))
  (`KismetArrayLibrary.Array_AddUnique` (`self.TurnOrder`) Unit)
  (`self.StartTurn`))

(event `StartTurn`
  (bind _output (`|GetArrayItem` (`self.TurnOrder`)))
  (bind _bp_combatcomponent (`/Game/Blueprints/Characters/Unit/BP_UnitBase.BP_CombatComponent` _output))
  (`/Engine/EditorBlueprintResources/StandardMacros.DoOnce` false :!label _label
    (:`Completed`
      (if (`KismetArrayLibrary.Array_IsValidIndex` (`self.TurnOrder`))
        (`/Game/Blueprints/Characters/Unit/BP_CombatComponent.StartUnitTurn` _bp_combatcomponent)
        (set `self.CurrentUnit` _output)
        (add `/Game/Blueprints/Characters/Unit/BP_CombatComponent.TurnEnded` _bp_combatcomponent (`|CreateDelegate` :!event `ReadyNextTurn`))
        (`KismetArrayLibrary.Array_Remove` (`self.TurnOrder`))
        (else
          (`self.ReadyNextTurn`))))))

(event `ReadyNextTurn`
  (`|ExecutionSequence`
    (:`then_0`
      (goto _label :!via `Reset`))
    (:`then_1`
      (if (`KismetArrayLibrary.Array_IsValidIndex` (`self.TurnOrder`))
        (`self.StartTurn`)))))

(fn `RandomizeTurnOrder`
  (bind _outactors (`GameplayStatics.GetAllActorsOfClass` "/Game/Blueprints/Characters/Unit/BP_UnitBase.BP_UnitBase_C"))
  (for _array_element _outactors
    (bind _output_get (set `/Game/Blueprints/Characters/Unit/BP_CombatComponent.Speed` (`KismetMathLibrary.RandomFloatInRange` 0.0 50.0) (`/Game/Blueprints/Characters/Unit/BP_UnitBase.BP_CombatComponent` _array_element)))
    (`KismetSystemLibrary.PrintText` (`/Game/Blueprints/Characters/Unit/BP_UnitBase.Name` _array_element))
    (`KismetSystemLibrary.PrintString` (`KismetStringLibrary.Conv_DoubleToString` _output_get))))

(fn `SpawnAllCharacters`
  (bind _outactors (`GameplayStatics.GetAllActorsOfClass` "/Game/Blueprints/Characters/Unit/BP_BattlePosition.BP_BattlePosition_C"))
  (for _array_element _outactors
    (`/Game/Blueprints/Characters/Unit/BP_BattlePosition.SpawnUnit` _array_element)))

(fn `UserConstructionScript`)