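; BP_DynamicCamera is a spring-arm camera actor that can attach to a target actor and orbit.
; SetOrbit toggles RotatingMovement's spin and the spring arm's yaw inheritance, resetting actor rotation when orbiting stops.
; SetDynamicLocation snaps the camera onto a valid actor's location through attachment and copies its rotation.
; The Vector input is unused, as the interpolated move toward a target location is disconnected and never runs.
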(event `self.ReceiveTick`
  (params (DeltaSeconds :type "Float (single-precision)")))

(event `/Game/Blueprints/Characters/BPI_DynamicCamera.SetOrbit`
  (params (IsOrbitting :type Boolean))
  (set `RotatingMovementComponent.RotationRate` (`KismetMathLibrary.SelectRotator` (struct :`Yaw` 10.0) (struct) IsOrbitting) (`self.RotatingMovement`))
  (bind _output_get (set `SpringArmComponent.bInheritYaw` IsOrbitting (`self.SpringArm`)))
  (if (not _output_get)
    (`self.K2_SetActorRotation` (struct))))

(event `/Game/Blueprints/Characters/BPI_DynamicCamera.SetDynamicLocation`
  (params (Actor :type "Actor Object Reference") (Vector :type "Vector Structure"))
  (`/Engine/EditorBlueprintResources/StandardMacros.IsValid` Actor
    (:`Is Valid`
      (`self.K2_AttachToActor` Actor "None" "SnapToTarget" "KeepWorld" "KeepWorld")
      (`self.K2_SetActorRotation` (`self.K2_GetActorRotation` Actor)))))

(fn `UserConstructionScript`)