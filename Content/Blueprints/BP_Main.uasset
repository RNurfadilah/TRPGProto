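; BP_Main is a player-controlled camera rig that pans, rotates and zooms on a spring arm.
; Enhanced Input events update desired location, yaw and clamped arm length, with panning relative to facing and rotation stepped per press.
; Tick smoothly interpolates toward those targets.
; BeginPlay adds the mapping context, seeds location and zoom from current values (rotation keeps its default) and shows the WBD_DebugTab widget.
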(event `EnhancedInput|/Game/Inputs/Actions/IA_CameraZoom`
  (params (ActionValue :type "Float (double-precision)") (ElapsedSeconds :type "Float (double-precision)") (TriggeredSeconds :type "Float (double-precision)") (InputAction :type "InputAction Object Reference" :default "/Game/Inputs/Actions/IA_CameraZoom.IA_CameraZoom"))
  ;[1 1 1] Comment
  (:`Triggered`
    (set `self.DesiredZoom` (`KismetMathLibrary.FClamp` (+ (* ActionValue (`self.ZoomSpeed`)) (`self.DesiredZoom`)) (`self.ZoomMin`) (`self.ZoomMax`)))))

(event `self.ReceiveBeginPlay`
  (`|ExecutionSequence`
    (:`then_0`
      (`self.EnhanceInputConstruct`))
    (:`then_1`
      (`self.StartingCameraPosition`))
    (:`then_2`
      (`self.StartingWidget`))))

(event `EnhancedInput|/Game/Inputs/Actions/IA_CameraMovement`
  (params (ActionValue :type "Vector2D Structure") (ElapsedSeconds :type "Float (double-precision)") (TriggeredSeconds :type "Float (double-precision)") (InputAction :type "InputAction Object Reference" :default "/Game/Inputs/Actions/IA_CameraMovement.IA_CameraMovement"))
  (bind _desiredlocation (`self.DesiredLocation`))
  ;[1 1 1] Comment
  (:`Triggered`
    (set `self.DesiredLocation` (+ (* (* ActionValue_X (`self.LocationSpeed`)) (`self.GetActorRightVector`)) _desiredlocation))
    (set `self.DesiredLocation` (+ _desiredlocation (* (`self.GetActorForwardVector`) (* (`self.LocationSpeed`) ActionValue_Y))))))

(event `self.ReceiveTick`
  (params (DeltaSeconds :type "Float (single-precision)"))
  (`|ExecutionSequence`
    (:`then_0`
      (`self.EnhanceInputCameraZoom` DeltaSeconds))
    (:`then_1`
      (`self.EnhanceInputCameraMovement` DeltaSeconds))
    (:`then_2`
      (`self.EnhanceInputCameraRotation` DeltaSeconds))))

(event `EnhancedInput|/Game/Inputs/Actions/IA_CameraRotate`
  (params (ActionValue :type "Float (double-precision)") (ElapsedSeconds :type "Float (double-precision)") (TriggeredSeconds :type "Float (double-precision)") (InputAction :type "InputAction Object Reference" :default "/Game/Inputs/Actions/IA_CameraRotate.IA_CameraRotate"))
  ;[1 1 1] Comment
  (:`Started`
    (set `self.DesiredRotation` (`KismetMathLibrary.ComposeRotators` (`self.DesiredRotation`) (`KismetMathLibrary.MakeRotator` 0.0 0.0 (* ActionValue (`self.RotationSpeed`)))))))

(fn `EnhanceInputCameraMovement`
  (params (DeltaTime :type "Float (double-precision)"))
  (`self.K2_SetActorLocation` (`KismetMathLibrary.VInterpTo` (`self.K2_GetActorLocation`) (`self.DesiredLocation`) DeltaTime (`self.LocationInterp`))))

(fn `EnhanceInputCameraRotation`
  (params (DeltaTime :type "Float (double-precision)"))
  (`self.K2_SetActorRotation` (`KismetMathLibrary.RInterpTo` (`self.K2_GetActorRotation`) (`self.DesiredRotation`) DeltaTime (`self.RotationInterp`))))

(fn `EnhanceInputCameraZoom`
  (params (DeltaTime :type "Float (double-precision)"))
  (bind _springarm (`self.SpringArm`))
  (set `SpringArmComponent.TargetArmLength` (`KismetMathLibrary.FInterpTo` (`SpringArmComponent.TargetArmLength` _springarm) (`self.DesiredZoom`) DeltaTime (`self.ZoomInterp`)) _springarm))

(fn `EnhanceInputConstruct`
  (bind _asplayer_controller (cast `PlayerController` (`self.GetController`)))
  (bind _returnvalue (pcsubsystem `EnhancedInputLocalPlayerSubsystem` _asplayer_controller))
  (`/Engine/EditorBlueprintResources/StandardMacros.IsValid` _returnvalue
    (:`Is Valid`
      (`EnhancedInputSubsystemInterface.AddMappingContext` _returnvalue "/Game/Inputs/IC_Default.IC_Default" 0 (struct)))))

(fn `StartingCameraPosition`
  (`|ExecutionSequence`
    (:`then_0`
      (set `self.DesiredLocation` (`self.K2_GetActorLocation`)))
    (:`then_1`
      (set `self.DesiredZoom` (`SpringArmComponent.TargetArmLength` (`self.SpringArm`))))
    (:`then_2`
      (set `self.DesiredRotation` (`self.DesiredRotation`)))))

(fn `StartingWidget`
  (bind _returnvalue (`|CreateWidget` "/Game/UIs/DebugMenu/WBD_DebugTab.WBD_DebugTab_C"))
  (`UserWidget.AddToViewport` _returnvalue 0)
  (`/Game/UIs/DebugMenu/WBD_DebugTab.SetHighlightedTab` _returnvalue))

(fn `UserConstructionScript`)