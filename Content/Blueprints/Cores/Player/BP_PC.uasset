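; Player controller for grid-based tactical battles that creates the battle HUD and drives unit movement and spell targeting with the mouse.
; Each tick it resolves the hovered unit or tile, previewing paths within the active player unit's reach.
; Clicking, or dragging across tiles, either moves the active unit or validates an ally/enemy target within spell range.
; Two grid pathfinders report through completion events, with tile states highlighting hover, reach, path and range.
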(event `self.ReceiveBeginPlay`
  (set `self.bShowMouseCursor` true)
  (bind _returnvalue (`GameplayStatics.GetActorOfClass` "/Game/Blueprints/Cores/Grid/BP_Grid.BP_Grid_C"))
  (set `self.Grid` _returnvalue)
  (bind _returnvalue_2 (`|CreateWidget` "/Game/UIs/CombatWidget/WBP_BattleHUD.WBP_BattleHUD_C"))
  (bind _output_get (set `self.BattleHUD` _returnvalue_2))
  (`UserWidget.AddToViewport` _output_get 0))

(event `self.ReceiveTick`
  (params (DeltaSeconds :type "Float (single-precision)"))
  (`self.UpdateTileAndUnitUnderCursor`))

(event `EnhancedInput|/Game/Inputs/Actions/IA_PlayerAction`
  (params (ActionValue :type Boolean) (ElapsedSeconds :type "Float (double-precision)") (TriggeredSeconds :type "Float (double-precision)") (InputAction :type "InputAction Object Reference" :default "/Game/Inputs/Actions/IA_PlayerAction.IA_PlayerAction"))
  (bind _hoveredtile (`self.HoveredTile`))
  (:`Started`
    (`self.UpdateTileAndUnitUnderCursor`)
    (set `self.IsLeftClickDown` true)
    (if (`self.IsSelectingTarget`) :!label _label
      (`self.Select Unit for Attack` _hoveredtile)
      (else
        (`self.MoveUnitOnGrid` _hoveredtile))))
  (:`Completed`
    (set `self.IsLeftClickDown` false)))

(event `OnHoveredTileChanged`
  (if (`self.IsLeftClickDown`)
    (goto _label)))

(fn `GenerateReachable`
  (locals (MaxPathLength :type Integer :default 5) (DelayBetweenItteration :type "Float (double-precision)") (MaxMsPerFrame :type "Float (double-precision)") (IncludeDiagonal :type Boolean))
  (bind _activeunit (`self.ActiveUnit`))
  (`/Game/Blueprints/Cores/Grid/BP_Grid.ClearStateFromTiles` (`self.Grid`) "NewEnumerator7")
  (set `self.IsMoveUnit` false)
  (add `/Game/Blueprints/Cores/Grid/BP_GridPathFinding.OnPathFindingCompleted` (`/Game/Blueprints/Cores/Grid/BP_Grid.GridPathFinding_Reachables` (`self.Grid`)) (`|CreateDelegate` :!event `On Pathfinding Completed`))
  (`/Engine/EditorBlueprintResources/StandardMacros.IsValid` (`self.ActiveUnit`)
    (:`Is Valid`
      (add `/Game/Blueprints/Characters/Unit/BP_UnitBase.OnUnitStartWalking` _activeunit (`|CreateDelegate` :!event `OnUnitStartWalking`))
      (add `/Game/Blueprints/Characters/Unit/BP_UnitBase.OnUnitFinishedWalking` _activeunit (`|CreateDelegate` :!event `OnUnitFinishWalking`))
      (`/Game/Blueprints/Cores/Grid/BP_GridPathFinding.Find Path` (`/Game/Blueprints/Cores/Grid/BP_Grid.GridPathFinding_Reachables` (`self.Grid`)) (`self.ActiveTile`) (make `IntPoint` -999 -999) (`local.IncludeDiagonal`) (`local.DelayBetweenItteration`) (`local.MaxMsPerFrame`) true (`/Game/Blueprints/Characters/Unit/BP_UnitBase.PathCurrent` (`self.ActiveUnit`))))
    (:`Is Not Valid`
      (`/Game/Blueprints/Cores/Grid/BP_GridPathFinding.Find Path` (`/Game/Blueprints/Cores/Grid/BP_Grid.GridPathFinding_Reachables` (`self.Grid`)) (`self.ActiveTile`) (make `IntPoint` -999 -999) (`local.IncludeDiagonal`) (`local.DelayBetweenItteration`) (`local.MaxMsPerFrame`) true (`local.MaxPathLength`)))))

(fn `GetTargetUnitAndTile`
  (params (Index :type "IntPoint Structure"))
  (returns (HideGrid :type Boolean))
  (bind _activeunit (`self.ActiveUnit`))
  (bind _returnvalue (`KismetMathLibrary.ClassIsChildOf` (`GameplayStatics.GetObjectClass` (`self.SelectedUnit`)) "/Game/Blueprints/Characters/Unit/Enemies/BP_EnemyUnitBase.BP_EnemyUnitBase_C"))
  (bind (_value _returnvalue_2) (`BlueprintMapLibrary.Map_Find` (`/Game/Blueprints/Cores/Grid/BP_Grid.GridTiles` (`self.Grid`)) (`self.SelectedTile`)))
  (bind ((`Index_4_5E2C0430450732CA0015FF88F0AA0B90` _index) (`UnitOnTile_17_296A43A74D08FB5B42D4D6A68D6A09A4` _unitontile)) (break `/Game/Blueprints/Cores/Utility/S_TileData` _value))
  (`/Engine/EditorBlueprintResources/StandardMacros.IsValid` _activeunit
    (:`Is Valid`
      (bind _rangeindexes (`/Game/Blueprints/Characters/Unit/BP_CombatComponent.GetSpellRange` :`self` (`/Game/Blueprints/Characters/Unit/BP_UnitBase.BP_CombatComponent` _activeunit)))
      (if (`KismetArrayLibrary.Array_Contains` _rangeindexes (`local.Index`))
        (if (!= (`self.SelectedTile`) (`local.Index`))
          (set `self.SelectedTile` (`local.Index`))
          (if _returnvalue_2
            (`/Engine/EditorBlueprintResources/StandardMacros.IsValid` _unitontile
              (:`Is Valid`
                (set `self.SelectedUnit` _unitontile)
                (if (`/Game/Blueprints/Characters/Unit/BP_CombatComponent.IsTargettingEnemy` (`/Game/Blueprints/Characters/Unit/BP_UnitBase.BP_CombatComponent` (`self.ActiveUnit`)))
                  (if _returnvalue
                    (`self.OnSelectedUnitAsTarget` (`self.SelectedUnit`) (`self.SelectedTile`) :!label _label)
                    (return true))
                  (elif (not _returnvalue)
                    (goto _label))))
              (:`Is Not Valid`
                (return false)))
            (else
              (return false))))
        (else
          (return false))))))

(fn `GetUnitUnderCursor`
  (returns (Unit :type "/Game/Blueprints/Characters/Unit/BP_UnitBase Object Reference"))
  (bind (_hitresult _returnvalue) (`self.GetHitResultUnderCursorByChannel` "TraceTypeQuery5"))
  (if _returnvalue
    (bind _asbp_unit_base (cast `/Game/Blueprints/Characters/Unit/BP_UnitBase` (`.HitActor` (`GameplayStatics.BreakHitResult` _hitresult))))
    (return _asbp_unit_base)
    (else
      (bind _index (`/Game/Blueprints/Cores/Grid/BP_Grid.GetTileIndexUnderCursor` (`self.Grid`) 0))
      (return (`.UnitOnTile_17_296A43A74D08FB5B42D4D6A68D6A09A4` (break `/Game/Blueprints/Cores/Utility/S_TileData` (`BlueprintMapLibrary.Map_Find` (`/Game/Blueprints/Cores/Grid/BP_Grid.GridTiles` (`self.Grid`)) _index)))))))

(fn `MoveUnitOnGrid`
  (params (Index :type "IntPoint Structure"))
  (bind _activeunit (`self.ActiveUnit`))
  (`/Game/Blueprints/Cores/Grid/BP_Grid.ClearStateFromTiles` (`self.Grid`) "NewEnumerator4")
  (`/Engine/EditorBlueprintResources/StandardMacros.IsValid` _activeunit
    (:`Is Valid`
      (add `/Game/Blueprints/Characters/Unit/BP_UnitBase.OnUnitFinishedWalking` _activeunit (`|CreateDelegate` :!event `OnUnitFinishWalking`))
      (set `self.IsMoveUnit` true)
      (add `/Game/Blueprints/Cores/Grid/BP_GridPathFinding.OnPathFindingCompleted` (`/Game/Blueprints/Cores/Grid/BP_Grid.GridPathFinding` (`self.Grid`)) (`|CreateDelegate` :!event `On Pathfinding Completed`))
      (`/Game/Blueprints/Cores/Grid/BP_GridPathFinding.Find Path` (`/Game/Blueprints/Cores/Grid/BP_Grid.GridPathFinding` (`self.Grid`)) (`self.ActiveTile`) (`local.Index`) false 0.0 0.0 false (`/Game/Blueprints/Characters/Unit/BP_UnitBase.PathCurrent` (`self.ActiveUnit`))))))

(fn `On Hover Pathfinding Completed`
  (params (Path :type "Array of IntPoint Structure (by ref)"))
  (`/Game/Blueprints/Cores/Grid/BP_Grid.ClearStateFromTiles` (`self.Grid`) "NewEnumerator4")
  (for _array_element Path
    (`/Game/Blueprints/Cores/Grid/BP_Grid.AddStateToTile` (`self.Grid`) _array_element "NewEnumerator4")))

(fn `On Pathfinding Completed`
  (params (Path :type "Array of IntPoint Structure (by ref)"))
  (if (`self.IsMoveUnit`)
    (for _array_element Path
      (`/Game/Blueprints/Cores/Grid/BP_Grid.AddStateToTile` (`self.Grid`) _array_element "NewEnumerator4"))
    (`/Game/Blueprints/Characters/Unit/BP_UnitBase.MoveToPath` (`self.ActiveUnit`) Path)
    (else
      (for _array_element_2 Path
        (`/Game/Blueprints/Cores/Grid/BP_Grid.AddStateToTile` (`self.Grid`) _array_element_2 "NewEnumerator7")))))

(fn `OnPlayerUnitActive`
  (`self.ShowReachableTiles` (`/Game/Blueprints/Characters/Unit/BP_UnitBase.Index` (`self.ActiveUnit`))))

(fn `OnUnitFinishWalking`
  (params (Unit :type "/Game/Blueprints/Characters/Unit/BP_UnitBase Object Reference"))
  (bind _grid (`self.Grid`))
  (`/Game/Blueprints/Cores/Grid/BP_Grid.ClearStateFromTiles` _grid "NewEnumerator4")
  (`/Game/Blueprints/Cores/Grid/BP_Grid.ClearStateFromTiles` _grid "NewEnumerator0")
  (`self.GenerateReachable`))

(fn `OnUnitStartWalking`
  (params (Unit :type "/Game/Blueprints/Characters/Unit/BP_UnitBase Object Reference"))
  (`/Game/Blueprints/Cores/Grid/BP_Grid.ClearStateFromTiles` (`self.Grid`) "NewEnumerator7"))

(fn `Select Unit for Attack`
  (params (Index :type "IntPoint Structure"))
  (bind _hidegrid (`self.GetTargetUnitAndTile` Index))
  (if _hidegrid
    (`/Game/Blueprints/Cores/Grid/BP_Grid.ClearStateFromTiles` (`self.Grid`) "NewEnumerator8")))

(fn `SelectTileAndUnit`
  (params (Index :type "IntPoint Structure"))
  (`self.SetActiveTileAndUnit` Index)
  (`/Game/Blueprints/Cores/Grid/BP_Grid.ClearStateFromTiles` (`self.Grid`) "NewEnumerator4"))

(fn `SetActiveTileAndUnit`
  (params (Index :type "IntPoint Structure"))
  (locals (NewUnit :type "/Game/Blueprints/Characters/Unit/BP_UnitBase Object Reference"))
  (if (!= (`self.ActiveTile`) (`local.Index`))
    (`/Game/Blueprints/Cores/Grid/BP_Grid.RemoveStateToTile` (`self.Grid`) (`self.ActiveTile`) "NewEnumerator2")
    (set `self.ActiveTile` (`local.Index`))
    (`/Game/Blueprints/Cores/Grid/BP_Grid.AddStateToTile` (`self.Grid`) (`self.ActiveTile`) "NewEnumerator2")
    (else
      (`/Engine/EditorBlueprintResources/StandardMacros.IsValid` (`self.ActiveUnit`)
        (:`Is Not Valid`
          (`/Game/Blueprints/Cores/Grid/BP_Grid.RemoveStateToTile` (`self.Grid`) (`self.ActiveTile`) "NewEnumerator2")
          (set `self.ActiveTile` (make `IntPoint` -999 -999)))))))

(fn `ShowAttackPattern`
  (`/Game/Blueprints/Cores/Grid/BP_Grid.ClearStateFromTiles` (`self.Grid`) "NewEnumerator7")
  (`self.ShowSpellRangePattern`))

(fn `ShowReachableTiles`
  (params (Index :type "IntPoint Structure"))
  (`self.SetActiveTileAndUnit` Index)
  (`self.GenerateReachable`))

(fn `ShowSpellRangePattern`
  (bind _activeunit (`self.ActiveUnit`))
  (`/Game/Blueprints/Cores/Grid/BP_Grid.ClearStateFromTiles` (`self.Grid`) "NewEnumerator8")
  (if (`/Game/Blueprints/Cores/Grid/BP_Grid.IsIndexValid` (`self.Grid`) (`self.ActiveTile`))
    (`/Engine/EditorBlueprintResources/StandardMacros.IsValid` _activeunit
      (:`Is Valid`
        (bind _rangeindexes (`/Game/Blueprints/Characters/Unit/BP_CombatComponent.GetSpellRange` :`self` (`/Game/Blueprints/Characters/Unit/BP_UnitBase.BP_CombatComponent` _activeunit)))
        (for _array_element _rangeindexes
          (`/Game/Blueprints/Cores/Grid/BP_Grid.AddStateToTile` (`self.Grid`) _array_element "NewEnumerator8"))))))

(fn `UpdateTileAndUnitUnderCursor`
  (locals (NewIndex :type "IntPoint Structure"))
  (bind _hoveredunit (`self.HoveredUnit`))
  (bind _activeunit (`self.ActiveUnit`))
  (`|ExecutionSequence`
    (:`then_0`
      (bind _unit (`self.GetUnitUnderCursor`))
      (if (!= _unit (`self.HoveredUnit`))
        (set `self.HoveredUnit` _unit)))
    (:`then_1`
      (`/Engine/EditorBlueprintResources/StandardMacros.IsValid` _hoveredunit
        (:`Is Valid`
          (set `local.NewIndex` (`/Game/Blueprints/Characters/Unit/BP_UnitBase.Index` _hoveredunit)))
        (:`Is Not Valid`
          (bind _index (`/Game/Blueprints/Cores/Grid/BP_Grid.GetTileIndexUnderCursor` (`self.Grid`) 0))
          (set `local.NewIndex` _index)))
      (if (!= (`local.NewIndex`) (`self.HoveredTile`))
        (`/Game/Blueprints/Cores/Grid/BP_Grid.RemoveStateToTile` (`self.Grid`) (`self.HoveredTile`) "NewEnumerator1")
        (set `self.HoveredTile` (`local.NewIndex`))
        (if (and (`KismetMathLibrary.ClassIsChildOf` (`GameplayStatics.GetObjectClass` _activeunit) "/Game/Blueprints/Characters/Unit/Characters/BP_PlayerUnitBase.BP_PlayerUnitBase_C") (`KismetSystemLibrary.IsValid` _activeunit) (not (`self.IsMoveUnit`)) (not (`self.IsSelectingTarget`)))
          (bind _path (`/Game/Blueprints/Cores/Grid/BP_GridPathFinding.Find Path` (`/Game/Blueprints/Cores/Grid/BP_Grid.GridPathFinding_Reachables` (`self.Grid`)) (`self.ActiveTile`) (make `IntPoint` -999 -999) false 0.0 0.0 true (`/Game/Blueprints/Characters/Unit/BP_UnitBase.PathCurrent` (`self.ActiveUnit`))))
          (if (`KismetArrayLibrary.Array_Contains` _path (`self.HoveredTile`))
            (add `/Game/Blueprints/Cores/Grid/BP_GridPathFinding.OnPathFindingCompleted` (`/Game/Blueprints/Cores/Grid/BP_Grid.GridPathFinding` (`self.Grid`)) (`|CreateDelegate` :!event `On Hover Pathfinding Completed`))
            (`/Game/Blueprints/Cores/Grid/BP_GridPathFinding.Find Path` (`/Game/Blueprints/Cores/Grid/BP_Grid.GridPathFinding` (`self.Grid`)) (`self.ActiveTile`) (`self.HoveredTile`) false 0.0 0.0 false (`/Game/Blueprints/Characters/Unit/BP_UnitBase.PathCurrent` (`self.ActiveUnit`)))
            (`self.OnHoveredTileChanged`)
            (else
              (`/Game/Blueprints/Cores/Grid/BP_Grid.ClearStateFromTiles` (`self.Grid`) "NewEnumerator4")
              (`/Game/Blueprints/Cores/Grid/BP_Grid.AddStateToTile` (`self.Grid`) (`self.HoveredTile`) "NewEnumerator1")
              (`self.OnHoveredTileChanged`)))
          (else
            (`/Game/Blueprints/Cores/Grid/BP_Grid.AddStateToTile` (`self.Grid`) (`self.HoveredTile`) "NewEnumerator1")
            (`self.OnHoveredTileChanged`)))))))

(fn `UserConstructionScript`)