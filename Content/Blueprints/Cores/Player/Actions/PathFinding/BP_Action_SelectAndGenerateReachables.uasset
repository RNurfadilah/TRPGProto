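; Player action that shows the grid tiles reachable from the active tile as a highlighted tile state.
; Executing it clears the old state and runs the grid's reachables pathfinder, limited by the active unit's current path value, or a default maximum when no valid unit exists.
; Completion marks each returned tile.
; When the unit starts walking the highlights clear, and when it finishes they are regenerated.
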(fn `ExecuteAction`
  (params (Index :type "IntPoint Structure"))
  (`parent.ExecuteAction` Index)
  (`self.GenerateReachables`))

(fn `GenerateReachables`
  (bind _activeunit (`/Game/Blueprints/Cores/Player/BP_PlayerAction.ActiveUnit` (`self.BPPlayerAction`)))
  (`/Game/Blueprints/Cores/Grid/BP_Grid.ClearStateFromTiles` (`/Game/Blueprints/Cores/Player/BP_PlayerAction.Grid` (`self.BPPlayerAction`)) "NewEnumerator7")
  (add `/Game/Blueprints/Cores/Grid/BP_GridPathFinding.OnPathFindingCompleted` (`/Game/Blueprints/Cores/Grid/BP_Grid.GridPathFinding_Reachables` (`/Game/Blueprints/Cores/Player/BP_PlayerAction.Grid` (`self.BPPlayerAction`))) (`|CreateDelegate` :!event `OnPathfindingCompleted`))
  (`/Engine/EditorBlueprintResources/StandardMacros.IsValid` (`/Game/Blueprints/Cores/Player/BP_PlayerAction.ActiveUnit` (`self.BPPlayerAction`))
    (:`Is Valid`
      (add `/Game/Blueprints/Characters/Unit/BP_UnitBase.OnUnitStartWalking` _activeunit (`|CreateDelegate` :!event `OnUnitStartWalking`))
      (add `/Game/Blueprints/Characters/Unit/BP_UnitBase.OnUnitFinishedWalking` _activeunit (`|CreateDelegate` :!event `OnUnitFinishWalking`))
      (`/Game/Blueprints/Cores/Grid/BP_GridPathFinding.Find Path` (`/Game/Blueprints/Cores/Grid/BP_Grid.GridPathFinding_Reachables` (`/Game/Blueprints/Cores/Player/BP_PlayerAction.Grid` (`self.BPPlayerAction`))) (`/Game/Blueprints/Cores/Player/BP_PlayerAction.ActiveTile` (`self.BPPlayerAction`)) (make `IntPoint` -999 -999) (`self.IncludeDiagonal`) (`self.DelayBetweenItteration`) (`self.MaxMsPerFrame`) true (`/Game/Blueprints/Characters/Unit/BP_UnitBase.PathCurrent` (`/Game/Blueprints/Cores/Player/BP_PlayerAction.ActiveUnit` (`self.BPPlayerAction`)))))
    (:`Is Not Valid`
      (`/Game/Blueprints/Cores/Grid/BP_GridPathFinding.Find Path` (`/Game/Blueprints/Cores/Grid/BP_Grid.GridPathFinding_Reachables` (`/Game/Blueprints/Cores/Player/BP_PlayerAction.Grid` (`self.BPPlayerAction`))) (`/Game/Blueprints/Cores/Player/BP_PlayerAction.ActiveTile` (`self.BPPlayerAction`)) (make `IntPoint` -999 -999) (`self.IncludeDiagonal`) (`self.DelayBetweenItteration`) (`self.MaxMsPerFrame`) true (`self.MaxPathLength`)))))

(fn `OnPathfindingCompleted`
  (params (Path :type "Array of IntPoint Structure (by ref)"))
  (for _array_element Path
    (`/Game/Blueprints/Cores/Grid/BP_Grid.AddStateToTile` (`/Game/Blueprints/Cores/Player/BP_PlayerAction.Grid` (`self.BPPlayerAction`)) _array_element "NewEnumerator7")))

(fn `OnUnitFinishWalking`
  (params (Unit :type "/Game/Blueprints/Characters/Unit/BP_UnitBase Object Reference"))
  (`self.GenerateReachables`))

(fn `OnUnitStartWalking`
  (params (Unit :type "/Game/Blueprints/Characters/Unit/BP_UnitBase Object Reference"))
  (`/Game/Blueprints/Cores/Grid/BP_Grid.ClearStateFromTiles` (`/Game/Blueprints/Cores/Player/BP_PlayerAction.Grid` (`self.BPPlayerAction`)) "NewEnumerator7"))

(fn `UserConstructionScript`
  (`parent.UserConstructionScript`))