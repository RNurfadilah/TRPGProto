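; Player action that marks the valid neighbor tiles of a given grid tile, optionally including diagonals.
; ExecuteAction clears a tile state from the grid, asks GridPathFinding for the valid neighbors of the index, then applies that state to each one.
; On Destroyed it runs again with an out-of-range sentinel index, apparently to clear the marks when the action is removed.
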(event `self.ReceiveDestroyed`
  (`self.ExecuteAction` (make `IntPoint` -999 -999)))

(fn `ExecuteAction`
  (params (Index :type "IntPoint Structure"))
  (`/Game/Blueprints/Cores/Grid/BP_Grid.ClearStateFromTiles` (`/Game/Blueprints/Cores/Player/BP_PlayerAction.Grid` (`self.BPPlayerAction`)) "NewEnumerator3")
  (bind _newparam (`/Game/Blueprints/Cores/Grid/BP_GridPathFinding.GetValidTileNeighbors` (`/Game/Blueprints/Cores/Grid/BP_Grid.GridPathFinding` (`/Game/Blueprints/Cores/Player/BP_PlayerAction.Grid` (`self.BPPlayerAction`))) Index (`self.Include Diagonal`)))
  (for _array_element _newparam
    (`/Game/Blueprints/Cores/Grid/BP_Grid.AddStateToTile` (`/Game/Blueprints/Cores/Player/BP_PlayerAction.Grid` (`self.BPPlayerAction`)) (break `/Game/Blueprints/Cores/Utility/S_PathFindingData` _array_element) "NewEnumerator3")))

(fn `UserConstructionScript`
  (`parent.UserConstructionScript`))