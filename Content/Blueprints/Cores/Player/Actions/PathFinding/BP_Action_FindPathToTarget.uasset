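; BP_Action_FindPathToTarget is a grid player action that marks the path from the selected tile to a target tile.
; On execute, it clears one tile state grid-wide, asks the grid's pathfinding component for a path with optional diagonals, then applies that state to each returned tile.
; On destruction, it re-executes with an out-of-range sentinel index, which serves to clear the displayed path.
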(event `self.ReceiveDestroyed`
  (`self.ExecuteAction` (make `IntPoint` -999 -999)))

(fn `ExecuteAction`
  (params (Index :type "IntPoint Structure"))
  (`/Game/Blueprints/Cores/Grid/BP_Grid.ClearStateFromTiles` (`/Game/Blueprints/Cores/Player/BP_PlayerAction.Grid` (`self.BPPlayerAction`)) "NewEnumerator4")
  (bind _path (`/Game/Blueprints/Cores/Grid/BP_GridPathFinding.FindPath` (`/Game/Blueprints/Cores/Grid/BP_Grid.GridPathFinding` (`/Game/Blueprints/Cores/Player/BP_PlayerAction.Grid` (`self.BPPlayerAction`))) (`/Game/Blueprints/Cores/Player/BP_PlayerAction.SelectedTile` (`self.BPPlayerAction`)) Index (`self.Include Diagonal`)))
  (for _array_element _path
    (`/Game/Blueprints/Cores/Grid/BP_Grid.AddStateToTile` (`/Game/Blueprints/Cores/Player/BP_PlayerAction.Grid` (`self.BPPlayerAction`)) _array_element "NewEnumerator4")))

(fn `UserConstructionScript`
  (`parent.UserConstructionScript`))