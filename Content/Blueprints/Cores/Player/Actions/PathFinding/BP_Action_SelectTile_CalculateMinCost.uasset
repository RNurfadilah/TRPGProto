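; Player grid action that fills pathfinding data with each tile's minimum cost to the player's active tile.
; On execute it runs the parent action, clears generated pathfinding data and stops there if the active tile is invalid.
; Otherwise it registers every grid tile as discovered, with zero cost from start and the estimated cost to the active tile, honoring the diagonals setting.
; No path search runs here, only this per-tile estimate.
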(fn `ExecuteAction`
  (params (Index :type "IntPoint Structure"))
  (bind _bpplayeraction (`self.BPPlayerAction`))
  (bind _bpplayeraction_2 (`self.BPPlayerAction`))
  (bind _grid (`/Game/Blueprints/Cores/Player/BP_PlayerAction.Grid` _bpplayeraction))
  (`parent.ExecuteAction` Index)
  (`/Game/Blueprints/Cores/Grid/BP_GridPathFinding.ClearGeneratedData` (`/Game/Blueprints/Cores/Grid/BP_Grid.GridPathFinding` (`/Game/Blueprints/Cores/Player/BP_PlayerAction.Grid` (`self.BPPlayerAction`))))
  (if (`/Game/Blueprints/Cores/Grid/BP_Grid.IsIndexValid` (`/Game/Blueprints/Cores/Player/BP_PlayerAction.Grid` _bpplayeraction_2) (`/Game/Blueprints/Cores/Player/BP_PlayerAction.ActiveTile` _bpplayeraction_2))
    (bind _keys (`BlueprintMapLibrary.Map_Keys` (`/Game/Blueprints/Cores/Grid/BP_Grid.GridTiles` _grid)))
    (for _array_element _keys
      (`/Game/Blueprints/Cores/Grid/BP_GridPathFinding.DiscoverTile` (`/Game/Blueprints/Cores/Grid/BP_Grid.GridPathFinding` (`/Game/Blueprints/Cores/Player/BP_PlayerAction.Grid` (`self.BPPlayerAction`))) (make `/Game/Blueprints/Cores/Utility/S_PathFindingData` _array_element 1 0 (`/Game/Blueprints/Cores/Grid/BP_GridPathFinding.GetMinimunCostBetweenTwoTiles` (`/Game/Blueprints/Cores/Grid/BP_Grid.GridPathFinding` _grid) _array_element (`/Game/Blueprints/Cores/Player/BP_PlayerAction.ActiveTile` _bpplayeraction) (`self.IncludeDiagonals`)))))))

(fn `UserConstructionScript`
  (`parent.UserConstructionScript`))