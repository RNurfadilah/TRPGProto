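; Player action that moves the active unit along a pathfound route on the tile grid.
; ExecuteAction clears a tile state, then requests a path from the active tile to the target, limited by the unit's current path length.
; When pathfinding completes, it marks the path tiles and starts the walk if that unit is still active, clearing two tile states once walking finishes.
; EndPlay re-runs the action with an off-grid sentinel index.
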(event `self.ReceiveEndPlay`
  (params (EndPlayReason :type "EEndPlayReason Enum" :default "Destroyed"))
  (`self.ExecuteAction` (make `IntPoint` -999 -999)))

(fn `ExecuteAction`
  (params (Index :type "IntPoint Structure"))
  (`/Game/Blueprints/Cores/Grid/BP_Grid.ClearStateFromTiles` (`/Game/Blueprints/Cores/Player/BP_PlayerAction.Grid` (`self.BPPlayerAction`)) "NewEnumerator4")
  (bind _output_get (set `self.CurrentUnit` (`/Game/Blueprints/Cores/Player/BP_PlayerAction.ActiveUnit` (`self.BPPlayerAction`))))
  (`/Engine/EditorBlueprintResources/StandardMacros.IsValid` _output_get
    (:`Is Valid`
      (add `/Game/Blueprints/Characters/Unit/BP_UnitBase.OnUnitFinishedWalking` (`self.CurrentUnit`) (`|CreateDelegate` :!event `On Unit Finished Walking`))
      (add `/Game/Blueprints/Cores/Grid/BP_GridPathFinding.OnPathFindingCompleted` (`/Game/Blueprints/Cores/Grid/BP_Grid.GridPathFinding` (`/Game/Blueprints/Cores/Player/BP_PlayerAction.Grid` (`self.BPPlayerAction`))) (`|CreateDelegate` :!event `On Path Finding Completed`))
      (`/Game/Blueprints/Cores/Grid/BP_GridPathFinding.Find Path` (`/Game/Blueprints/Cores/Grid/BP_Grid.GridPathFinding` (`/Game/Blueprints/Cores/Player/BP_PlayerAction.Grid` (`self.BPPlayerAction`))) (`/Game/Blueprints/Cores/Player/BP_PlayerAction.ActiveTile` (`self.BPPlayerAction`)) (`local.Index`) false 0.0 0.0 false (`/Game/Blueprints/Characters/Unit/BP_UnitBase.PathCurrent` (`/Game/Blueprints/Cores/Player/BP_PlayerAction.ActiveUnit` (`self.BPPlayerAction`)))))))

(fn `On Path Finding Completed`
  (params (Path :type "Array of IntPoint Structure"))
  (`/Engine/EditorBlueprintResources/StandardMacros.IsValid` (`self.CurrentUnit`)
    (:`Is Valid`
      (if (== (`self.CurrentUnit`) (`/Game/Blueprints/Cores/Player/BP_PlayerAction.ActiveUnit` (`self.BPPlayerAction`)))
        (for _array_element (`local.Path`)
          (`/Game/Blueprints/Cores/Grid/BP_Grid.AddStateToTile` (`/Game/Blueprints/Cores/Player/BP_PlayerAction.Grid` (`self.BPPlayerAction`)) _array_element "NewEnumerator4"))
        (`/Game/Blueprints/Characters/Unit/BP_UnitBase.MoveToPath` (`self.CurrentUnit`) (`local.Path`))))))

(fn `On Unit Finished Walking`
  (params (Unit :type "/Game/Blueprints/Characters/Unit/BP_UnitBase Object Reference"))
  (bind _grid (`/Game/Blueprints/Cores/Player/BP_PlayerAction.Grid` (`self.BPPlayerAction`)))
  (if (== Unit (`self.CurrentUnit`))
    (`/Game/Blueprints/Cores/Grid/BP_Grid.ClearStateFromTiles` _grid "NewEnumerator4")
    (`/Game/Blueprints/Cores/Grid/BP_Grid.ClearStateFromTiles` _grid "NewEnumerator7")))

(fn `UserConstructionScript`
  (`parent.UserConstructionScript`))