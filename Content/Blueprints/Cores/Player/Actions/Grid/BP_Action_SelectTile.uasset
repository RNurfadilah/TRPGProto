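; Player grid action that toggles which tile is selected on the grid.
; ExecuteAction moves the selection state from the previously selected tile to the given index through the player action's Grid and stores it as SelectedTile.
; Passing the already selected tile clears the selection to a -999 sentinel index.
; On Destroyed, it executes with that sentinel so the previous tile loses its selected state.
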(event `self.ReceiveDestroyed`
  (`self.ExecuteAction` (make `IntPoint` -999 -999)))

(fn `ExecuteAction`
  (params (Index :type "IntPoint Structure"))
  (bind _bpplayeraction (`self.BPPlayerAction`))
  (bind _bpplayeraction_2 (`self.BPPlayerAction`))
  (bind _bpplayeraction_3 (`self.BPPlayerAction`))
  (if (!= (`/Game/Blueprints/Cores/Player/BP_PlayerAction.SelectedTile` (`self.BPPlayerAction`)) (`local.Index`))
    (`/Game/Blueprints/Cores/Grid/BP_Grid.RemoveStateToTile` (`/Game/Blueprints/Cores/Player/BP_PlayerAction.Grid` _bpplayeraction_2) (`/Game/Blueprints/Cores/Player/BP_PlayerAction.SelectedTile` _bpplayeraction_2) "NewEnumerator2")
    (set `/Game/Blueprints/Cores/Player/BP_PlayerAction.SelectedTile` (`local.Index`) (`self.BPPlayerAction`))
    (`/Game/Blueprints/Cores/Grid/BP_Grid.AddStateToTile` (`/Game/Blueprints/Cores/Player/BP_PlayerAction.Grid` _bpplayeraction) (`/Game/Blueprints/Cores/Player/BP_PlayerAction.SelectedTile` _bpplayeraction) "NewEnumerator2")
    (else
      (`/Game/Blueprints/Cores/Grid/BP_Grid.RemoveStateToTile` (`/Game/Blueprints/Cores/Player/BP_PlayerAction.Grid` _bpplayeraction_3) (`/Game/Blueprints/Cores/Player/BP_PlayerAction.SelectedTile` _bpplayeraction_3) "NewEnumerator2")
      (set `/Game/Blueprints/Cores/Player/BP_PlayerAction.SelectedTile` (make `IntPoint` -999 -999) (`self.BPPlayerAction`)))))

(fn `UserConstructionScript`
  (`parent.UserConstructionScript`))