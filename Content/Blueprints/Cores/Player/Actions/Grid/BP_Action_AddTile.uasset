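; Player grid action that adds a tile at a given index on the grid.
; ExecuteAction acts only when the index is not already valid in the grid, so existing tiles are left untouched.
; It passes a fixed tile type to AddGridTile, with location and rotation derived from the index and scale taken from the grid's GetTileScan.
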(fn `ExecuteAction`
  (params (Index :type "IntPoint Structure"))
  (bind _index (`local.Index`))
  (bind _grid (`/Game/Blueprints/Cores/Player/BP_PlayerAction.Grid` (`self.BPPlayerAction`)))
  (if (not (`/Game/Blueprints/Cores/Grid/BP_Grid.IsIndexValid` (`/Game/Blueprints/Cores/Player/BP_PlayerAction.Grid` (`self.BPPlayerAction`)) Index))
    (`/Game/Blueprints/Cores/Grid/BP_Grid.AddGridTile` (`/Game/Blueprints/Cores/Player/BP_PlayerAction.Grid` (`self.BPPlayerAction`)) (make `/Game/Blueprints/Cores/Utility/S_TileData` (`local.Index`) "NewEnumerator1" (`KismetMathLibrary.MakeTransform` (`/Game/Blueprints/Cores/Grid/BP_Grid.GetTileLocationFromGridIndex` _grid _index) (`/Game/Blueprints/Cores/Grid/BP_Grid.GetTileRotationFromGridIndex` _grid _index) (`/Game/Blueprints/Cores/Grid/BP_Grid.GetTileScan` _grid))))))

(fn `UserConstructionScript`
  (`parent.UserConstructionScript`))