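; Player grid action that raises or lowers a single tile's height on the grid.
; ExecuteAction validates the tile index, reads its stored data, then re-adds the tile with its location moved one grid tile size along Z, up or down according to the Increase flag.
; Tile type, rotation, scale and states carry over unchanged.
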(fn `ExecuteAction`
  (params (Index :type "IntPoint Structure"))
  (locals (Data :type "/Game/Blueprints/Cores/Utility/S_TileData Structure"))
  (bind _data (`local.Data`))
  (bind (_grid_tile_size_x _grid_tile_size_y _grid_tile_size_z) (`KismetMathLibrary.BreakVector` (`/Game/Blueprints/Cores/Grid/BP_Grid.Grid Tile Size` (`/Game/Blueprints/Cores/Player/BP_PlayerAction.Grid` (`self.BPPlayerAction`)))))
  (if (`/Game/Blueprints/Cores/Grid/BP_Grid.IsIndexValid` (`/Game/Blueprints/Cores/Player/BP_PlayerAction.Grid` (`self.BPPlayerAction`)) Index)
    (set `local.Data` (`BlueprintMapLibrary.Map_Find` (`/Game/Blueprints/Cores/Grid/BP_Grid.GridTiles` (`/Game/Blueprints/Cores/Player/BP_PlayerAction.Grid` (`self.BPPlayerAction`))) (`local.Index`)))
    (`/Game/Blueprints/Cores/Grid/BP_Grid.AddGridTile` (`/Game/Blueprints/Cores/Player/BP_PlayerAction.Grid` (`self.BPPlayerAction`)) (make `/Game/Blueprints/Cores/Utility/S_TileData` (break `/Game/Blueprints/Cores/Utility/S_TileData` _data) (`.TileType_9_106D6E0E42F9FFF0D96DB0BBF5AB807D` (break `/Game/Blueprints/Cores/Utility/S_TileData` _data)) (`KismetMathLibrary.MakeTransform` (+ (.location (`.Transform_8_1A7B87B34336F36EDDECB69D5BF0102F` (break `/Game/Blueprints/Cores/Utility/S_TileData` _data))) (`KismetMathLibrary.MakeVector` 0.0 0.0 (* _grid_tile_size_z (`KismetMathLibrary.SelectFloat` 1.0 -1.0 (`self.Increase`))))) (.rotation (`.Transform_8_1A7B87B34336F36EDDECB69D5BF0102F` (break `/Game/Blueprints/Cores/Utility/S_TileData` _data))) (.scale (`.Transform_8_1A7B87B34336F36EDDECB69D5BF0102F` (break `/Game/Blueprints/Cores/Utility/S_TileData` _data)))) (`.TileStates_14_E1FC77214B918AC789E77C9955B2159B` (break `/Game/Blueprints/Cores/Utility/S_TileData` _data))))))

(fn `UserConstructionScript`
  (`parent.UserConstructionScript`))