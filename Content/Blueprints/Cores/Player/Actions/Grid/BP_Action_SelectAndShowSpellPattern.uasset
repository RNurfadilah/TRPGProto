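; Player grid action that highlights the active unit's spell range pattern on the grid when executed.
; After running the parent action, it clears the range tile state from the grid.
; If the active tile and unit are valid, it gets the spell range from the unit's combat component in non-AI mode and adds that state to each returned tile.
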(fn `ExecuteAction`
  (params (Index :type "IntPoint Structure"))
  (`parent.ExecuteAction` Index)
  (`self.ShowSpellRangePattern`))

(fn `ShowSpellRangePattern`
  (bind _bpplayeraction (`self.BPPlayerAction`))
  (bind _activeunit (`/Game/Blueprints/Cores/Player/BP_PlayerAction.ActiveUnit` (`self.BPPlayerAction`)))
  (`/Game/Blueprints/Cores/Grid/BP_Grid.ClearStateFromTiles` (`/Game/Blueprints/Cores/Player/BP_PlayerAction.Grid` (`self.BPPlayerAction`)) "NewEnumerator8")
  (if (`/Game/Blueprints/Cores/Grid/BP_Grid.IsIndexValid` (`/Game/Blueprints/Cores/Player/BP_PlayerAction.Grid` _bpplayeraction) (`/Game/Blueprints/Cores/Player/BP_PlayerAction.ActiveTile` _bpplayeraction))
    (`/Engine/EditorBlueprintResources/StandardMacros.IsValid` _activeunit
      (:`Is Valid`
        (bind _rangeindexes (`/Game/Blueprints/Characters/Unit/BP_CombatComponent.GetSpellRange` :`self` (`/Game/Blueprints/Characters/Unit/BP_UnitBase.BP_CombatComponent` _activeunit)))
        (for _array_element _rangeindexes
          (`/Game/Blueprints/Cores/Grid/BP_Grid.AddStateToTile` (`/Game/Blueprints/Cores/Player/BP_PlayerAction.Grid` (`self.BPPlayerAction`)) _array_element "NewEnumerator8"))))))

(fn `UserConstructionScript`
  (`parent.UserConstructionScript`))