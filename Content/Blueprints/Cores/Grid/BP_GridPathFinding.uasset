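; Grid pathfinder that runs A* over square or hex tiles to return a path to a target or, optionally, the tiles reachable within a maximum length.
; Neighbors must be walkable, unoccupied and within one tile height.
; A cost-sorted open list ranks tiles by cost plus heuristic, penalizing diagonal steps on ties.
; Searches run instantly or time-sliced with a delay and per-frame millisecond budget, firing update, clear and completion callbacks.
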(event `FindPathWithDelay`
  (`|ExecutionSequence`
    (:`then_0`
      (goto _label_3 :!via `Open`))
    (:`then_1`
      (set `self.LoopStartTime` (`GameplayStatics.GetRealTimeSeconds`) :!label _label)
      (if (> (`KismetArrayLibrary.Array_Length` (`self.DiscoveredTileIndexes`)) 0) :!label _label_2
        (bind _foundtargettile (`self.AnalizeNextDiscoveredTiles`))
        (if _foundtargettile
          (bind _path (`self.GeneratePath`))
          (`self.OnPathFindingCompleted` _path)
          (else
            (if (> (`self.MaxMsPerFrame`) 0.0)
              (if (< (- (`GameplayStatics.GetRealTimeSeconds`) (`self.LoopStartTime`)) (`self.MaxMsPerFrame`))
                (goto _label_2)
                (else
                  _)))
            (`KismetSystemLibrary.RetriggerableDelay` (`self.DelayBetweenIteratoin`))
            (`/Engine/EditorBlueprintResources/StandardMacros.Gate` true :!label _label_3
              (:`Exit`
                (goto _label)))))
        (else
          (`self.OnPathFindingCompleted` (select `bool` (`self.ReturnReachableTiles`) :`false` (`|MakeArray`) :`true` (`self.AnalizeTileIndexes`))))))))

(event `CloseDelayGate`
  (goto _label_3 :!via `Close`))

(fn `AnalizeNextDiscoveredTiles`
  (returns (FoundTargetTile :type Boolean))
  (bind _tilepathdata (`self.PullCheapesTileOutOfDiscoveredList`))
  (bind _output_get (set `self.CurrentDiscoveredTile` _tilepathdata))
  (`self.OnPathFindingDataUpdated` (`.Index_10_021D3DFB40F95023808975A0CD205470` (break `/Game/Blueprints/Cores/Utility/S_PathFindingData` _output_get)))
  (bind _neigbhors (`self.GetValidTileNeighbors` (`.Index_10_021D3DFB40F95023808975A0CD205470` (break `/Game/Blueprints/Cores/Utility/S_PathFindingData` (`self.CurrentDiscoveredTile`))) (`self.IncludeDiagonals`)))
  (set `self.CurrentNeighbors` _neigbhors)
  (while (> (`KismetArrayLibrary.Array_Length` (`self.CurrentNeighbors`)) 0)
    (bind _istargettile (`self.DiscoverNextNeighbor`))
    (if _istargettile
      (return true)))
  (return false))

(fn `ClearGeneratedData`
  (`BlueprintMapLibrary.Map_Clear` (`self.PathFindingData`))
  (`KismetArrayLibrary.Array_Clear` (`self.DiscoveredTileSortingCost`))
  (`KismetArrayLibrary.Array_Clear` (`self.DiscoveredTileIndexes`))
  (`KismetArrayLibrary.Array_Clear` (`self.AnalizeTileIndexes`))
  (`self.OnPathFindingDataCleared`))

(fn `DiscoverNextNeighbor`
  (returns (IsTargetTile :type Boolean))
  (locals (CostFromStart :type Integer) (IndexInDiscovered :type Integer :default 0))
  (bind _indexindiscovered (`local.IndexInDiscovered`))
  (bind _currentneighbor (`self.CurrentNeighbor`))
  (bind (_index _costoentertile) (break `/Game/Blueprints/Cores/Utility/S_PathFindingData` _currentneighbor))
  (set `self.CurrentNeighbor` (`|GetArrayItem` (`self.CurrentNeighbors`)))
  (`KismetArrayLibrary.Array_Remove` (`self.CurrentNeighbors`))
  (if (not (`KismetArrayLibrary.Array_Contains` (`self.AnalizeTileIndexes`) (`.Index_10_021D3DFB40F95023808975A0CD205470` (break `/Game/Blueprints/Cores/Utility/S_PathFindingData` (`self.CurrentNeighbor`)))))
    (set `local.CostFromStart` (+ (`.CosFromStart_12_3D38642B429114C0012CBDA898A886AF` (break `/Game/Blueprints/Cores/Utility/S_PathFindingData` (`self.CurrentDiscoveredTile`))) (`.CosToEnterTile_11_5A1FD0B849FD905C9E3A8489915E8F8D` (break `/Game/Blueprints/Cores/Utility/S_PathFindingData` (`self.CurrentNeighbor`)))))
    (if (<= (`local.CostFromStart`) (`self.MaxPathLength`))
      (bind _output_get (set `local.IndexInDiscovered` (`KismetArrayLibrary.Array_Find` (`self.DiscoveredTileIndexes`) (`.Index_10_021D3DFB40F95023808975A0CD205470` (break `/Game/Blueprints/Cores/Utility/S_PathFindingData` (`self.CurrentNeighbor`))))))
      (if (not (== _output_get -1))
        (bind _output_get_2 (set `self.CurrentNeighbor` (`BlueprintMapLibrary.Map_Find` (`self.PathFindingData`) (`.Index_10_021D3DFB40F95023808975A0CD205470` (break `/Game/Blueprints/Cores/Utility/S_PathFindingData` (`self.CurrentNeighbor`))))))
        (if (< (`local.CostFromStart`) (`.CosToEnterTile_11_5A1FD0B849FD905C9E3A8489915E8F8D` (break `/Game/Blueprints/Cores/Utility/S_PathFindingData` _output_get_2)))
          (`KismetArrayLibrary.Array_Remove` (`self.DiscoveredTileIndexes`) _indexindiscovered)
          (`KismetArrayLibrary.Array_Remove` (`self.DiscoveredTileSortingCost`) _indexindiscovered)
          (else
            (return false))))
      (`self.DiscoverTile` (make `/Game/Blueprints/Cores/Utility/S_PathFindingData` _index _costoentertile (`local.CostFromStart`) (`self.GetMinimunCostBetweenTwoTiles` (`.Index_10_021D3DFB40F95023808975A0CD205470` (break `/Game/Blueprints/Cores/Utility/S_PathFindingData` _currentneighbor)) (`self.TargetIndex`) (`self.IncludeDiagonals`)) (`.Index_10_021D3DFB40F95023808975A0CD205470` (break `/Game/Blueprints/Cores/Utility/S_PathFindingData` (`self.CurrentDiscoveredTile`)))))
      (if (`KismetMathLibrary.Equal_IntPointIntPoint` (`.Index_10_021D3DFB40F95023808975A0CD205470` (break `/Game/Blueprints/Cores/Utility/S_PathFindingData` (`self.CurrentNeighbor`))) (`self.TargetIndex`))
        (return true)
        (else
          (return false)))
      (else
        (return false)))
    (else
      (return false))))

(fn `DiscoverTile`
  (params (TilePathData :type "/Game/Blueprints/Cores/Utility/S_PathFindingData Structure"))
  (`BlueprintMapLibrary.Map_Add` (`self.PathFindingData`) (`.Index_10_021D3DFB40F95023808975A0CD205470` (break `/Game/Blueprints/Cores/Utility/S_PathFindingData` TilePathData)) TilePathData)
  (`self.InsertTileInDiscoveredArray` TilePathData)
  (`self.OnPathFindingDataUpdated` (struct)))

(fn `Find Path`
  (params (Start :type "IntPoint Structure") (Target :type "IntPoint Structure") (Diagonals :type Boolean) (DelayBetweenIteration :type "Float (double-precision)") (MaxMsPerFrame :type "Float (double-precision)") (ReturnReachables :type Boolean) (PathLength :type Integer))
  (returns (Path :type "Array of IntPoint Structure"))
  (bind _array (`|MakeArray`))
  (bind _returnvalue (select `bool` (`self.ReturnReachableTiles`) :`false` (`|MakeArray`) :`true` (`self.AnalizeTileIndexes`)))
  (set `self.StartIndex` Start)
  (set `self.TargetIndex` Target)
  (set `self.IncludeDiagonals` Diagonals)
  (set `self.DelayBetweenIteratoin` DelayBetweenIteration)
  (set `self.MaxMsPerFrame` MaxMsPerFrame)
  (set `self.ReturnReachableTiles` ReturnReachables)
  (set `self.MaxPathLength` PathLength)
  (`self.CloseDelayGate`)
  (`self.ClearGeneratedData`)
  (bind _isvalid (`self.IsInputDataValid`))
  (if _isvalid
    (`self.DiscoverTile` (make `/Game/Blueprints/Cores/Utility/S_PathFindingData` (`self.StartIndex`) 1 0 (`self.GetMinimunCostBetweenTwoTiles` (`self.StartIndex`) (`self.TargetIndex`) (`self.IncludeDiagonals`))))
    (if (<= (`self.DelayBetweenIteratoin`) 0.0)
      (while (> (`KismetArrayLibrary.Array_Length` (`self.DiscoveredTileIndexes`)) 0)
        (bind _foundtargettile (`self.AnalizeNextDiscoveredTiles`))
        (if _foundtargettile
          (bind _path (`self.GeneratePath`))
          (`self.OnPathFindingCompleted` _path)
          (return _path)))
      (`self.OnPathFindingCompleted` _returnvalue)
      (return _returnvalue)
      (else
        (`self.FindPathWithDelay`)
        (return (`|MakeArray`))))
    (else
      (`self.OnPathFindingCompleted` _array)
      (return _array))))

(fn `GeneratePath`
  (returns (Path :type "Array of IntPoint Structure"))
  (locals (Current :type "IntPoint Structure") (InvertedPath :type "Array of IntPoint Structure") (RET :type "Array of IntPoint Structure"))
  (bind _output_get (set `local.Current` (`self.TargetIndex`)))
  (while (!= _output_get (`self.StartIndex`))
    (`KismetArrayLibrary.Array_Add` (`local.InvertedPath`) (`local.Current`))
    (set `local.Current` (`.PreviousIndex_14_59EB1C484484F4B7443619A7C5DE6B8A` (break `/Game/Blueprints/Cores/Utility/S_PathFindingData` (`BlueprintMapLibrary.Map_Find` (`self.PathFindingData`) (`local.Current`))))))
  (bind (_arrayindex _arrayelement) (`/Engine/EditorBlueprintResources/StandardMacros.ReverseForEachLoop` (`local.InvertedPath`))
    (:`LoopBody`
      (`KismetArrayLibrary.Array_Add` (`local.RET`) _arrayelement))
    (:`Completed`
      (return (`local.RET`)))))

(fn `Get Tile Sorting Cost`
  (params (TileData :type "/Game/Blueprints/Cores/Utility/S_PathFindingData Structure (by ref)"))
  (returns (Cost :type Integer))
  (bind ((`Index_10_021D3DFB40F95023808975A0CD205470` _index) (`PreviousIndex_14_59EB1C484484F4B7443619A7C5DE6B8A` _previousindex)) (break `/Game/Blueprints/Cores/Utility/S_PathFindingData` TileData))
  (bind ((`CosFromStart_12_3D38642B429114C0012CBDA898A886AF` _cosfromstart) (`MinimumCostToTarget_13_B80A5E824DB644D421F8229013151D33` _minimumcosttotarget)) (break `/Game/Blueprints/Cores/Utility/S_PathFindingData` TileData))
  (return (+ (* (+ _cosfromstart _minimumcosttotarget) 2) (`KismetMathLibrary.Conv_BoolToInt` (`self.IsDiagonal` _index _previousindex)))))

(fn `GetMinimunCostBetweenTwoTiles`
  (params (Index1 :type "IntPoint Structure") (Index2 :type "IntPoint Structure") (Diagonals :type Boolean))
  (returns (MinCost :type Integer))
  (bind (_returnvalue_x _returnvalue_y) (break `IntPoint` (- (`local.Index1`) (`local.Index2`))))
  (bind (_returnvalue_x_2 _returnvalue_y_2) (break `IntPoint` (- (`local.Index1`) (`local.Index2`))))
  (bind (_returnvalue_x_3 _returnvalue_y_3) (break `IntPoint` (- (`local.Index1`) (`local.Index2`))))
  (bind (_returnvalue_x_4 _returnvalue_y_4) (break `IntPoint` (- (`local.Index1`) (`local.Index2`))))
  (bind _returnvalue (`KismetMathLibrary.Abs_Int` _returnvalue_x))
  (switch `/Game/Blueprints/Cores/Grid/GridShapes/E_GridShape` (`/Game/Blueprints/Cores/Grid/BP_Grid.Grid Shape` (`self.Grid`))
    (:`NewEnumerator1`
      (return (+ _returnvalue (`KismetMathLibrary.Max` (/ (- (`KismetMathLibrary.Abs_Int` _returnvalue_y) _returnvalue) 2)))))
    (:`NewEnumerator2`
      (if (`self.IncludeDiagonals`)
        (return (`KismetMathLibrary.Max` (`KismetMathLibrary.Abs_Int` _returnvalue_x_2) (`KismetMathLibrary.Abs_Int` _returnvalue_y_2)))
        (else
          (return (+ (`KismetMathLibrary.Abs_Int` _returnvalue_x_4) (`KismetMathLibrary.Abs_Int` _returnvalue_y_4))))))
    (:`NewEnumerator3`
      (if (`self.IncludeDiagonals`)
        (return (+ (`KismetMathLibrary.Abs_Int` _returnvalue_x_3) (`KismetMathLibrary.Abs_Int` _returnvalue_y_3)))))))

(fn `GetNeighborIndexesForHexagon`
  (params (Index :type "IntPoint Structure") (IncludeDiagonal :type Boolean))
  (returns (Neighbors :type "Array of IntPoint Structure"))
  (locals (RET :type "Array of IntPoint Structure"))
  (return (`|MakeArray` (+ (`local.Index`) (make `IntPoint` 1 1)) (+ (`local.Index`) (make `IntPoint` 0 2)) (+ (`local.Index`) (make `IntPoint` -1 1)) (+ (`local.Index`) (make `IntPoint` -1 -1)) (+ (`local.Index`) (make `IntPoint` 0 -2)) (+ (`local.Index`) (make `IntPoint` 1 -1)))))

(fn `GetNeighborIndexesForSquare`
  (params (Index :type "IntPoint Structure") (IncludeDiagonal :type Boolean))
  (returns (Neighbors :type "Array of IntPoint Structure"))
  (locals (RET :type "Array of IntPoint Structure"))
  (bind _array (`|MakeArray` (+ (`local.Index`) (make `IntPoint` 1)) (+ (`local.Index`) (make `IntPoint` 0 1)) (+ (`local.Index`) (make `IntPoint` -1)) (+ (`local.Index`) (make `IntPoint` 0 -1))))
  (if IncludeDiagonal
    (set `local.RET` _array)
    (`KismetArrayLibrary.Array_Append` (`local.RET`) (`|MakeArray` (+ (`local.Index`) (make `IntPoint` 1 1)) (+ (`local.Index`) (make `IntPoint` -1 1)) (+ (`local.Index`) (make `IntPoint` -1 -1)) (+ (`local.Index`) (make `IntPoint` 1 -1))))
    (return (`local.RET`))
    (else
      (return _array))))

(fn `GetTileNeighbors`
  (params (Index :type "IntPoint Structure") (IncludeDiagonal :type Boolean))
  (returns (Neighbors :type "Array of IntPoint Structure"))
  (switch `/Game/Blueprints/Cores/Grid/GridShapes/E_GridShape` (`/Game/Blueprints/Cores/Grid/BP_Grid.Grid Shape` (`self.Grid`))
    (:`NewEnumerator1`
      (return (`self.GetNeighborIndexesForHexagon` (`local.Index`) IncludeDiagonal)))
    (:`NewEnumerator2`
      (return (`self.GetNeighborIndexesForSquare` (`local.Index`) IncludeDiagonal)))))

(fn `GetValidTileNeighbors`
  (params (Index :type "IntPoint Structure") (IncludeDiagonal :type Boolean))
  (returns (Neigbhors :type "Array of /Game/Blueprints/Cores/Utility/S_PathFindingData Structure"))
  (locals (Data :type "/Game/Blueprints/Cores/Utility/S_TileData Structure") (InputData :type "/Game/Blueprints/Cores/Utility/S_TileData Structure") (RET :type "Array of /Game/Blueprints/Cores/Utility/S_PathFindingData Structure"))
  (bind (_data_index _data_tiletype _data_transform _data_tilestates _data_unitontile) (break `/Game/Blueprints/Cores/Utility/S_TileData` (`local.Data`)))
  (bind _data_index_2 (break `/Game/Blueprints/Cores/Utility/S_TileData` (`local.Data`)))
  (bind (_grid_tile_size_x _grid_tile_size_y _grid_tile_size_z) (`KismetMathLibrary.BreakVector` (`/Game/Blueprints/Cores/Grid/BP_Grid.Grid Tile Size` (`self.Grid`))))
  (set `local.InputData` (`BlueprintMapLibrary.Map_Find` (`/Game/Blueprints/Cores/Grid/BP_Grid.GridTiles` (`self.Grid`)) (`local.Index`)))
  (bind _neighbors (`self.GetTileNeighbors` (`local.Index`) (`local.IncludeDiagonal`)))
  (for _array_element _neighbors
    (bind _output_get (set `local.Data` (`BlueprintMapLibrary.Map_Find` (`/Game/Blueprints/Cores/Grid/BP_Grid.GridTiles` (`self.Grid`)) _array_element)))
    (if (`/Game/Blueprints/Cores/Utility/BFL_TileData.IsTileTypeWalkAble` (`.TileType_9_106D6E0E42F9FFF0D96DB0BBF5AB807D` (break `/Game/Blueprints/Cores/Utility/S_TileData` _output_get)))
      (if (not (`KismetSystemLibrary.IsValid` _data_unitontile))
        (if (<= (`KismetMathLibrary.Abs` (- (.z (.location (`.Transform_8_1A7B87B34336F36EDDECB69D5BF0102F` (break `/Game/Blueprints/Cores/Utility/S_TileData` (`local.Data`))))) (.z (.location (`.Transform_8_1A7B87B34336F36EDDECB69D5BF0102F` (break `/Game/Blueprints/Cores/Utility/S_TileData` (`local.InputData`))))))) _grid_tile_size_z)
          (`KismetArrayLibrary.Array_Add` (`local.RET`) (make `/Game/Blueprints/Cores/Utility/S_PathFindingData` _data_index_2 1 999999 999999 (`local.Index`)))))))
  (return (`local.RET`)))

(fn `InsertTileInDiscoveredArray`
  (params (TileData :type "/Game/Blueprints/Cores/Utility/S_PathFindingData Structure"))
  (locals (SortingCost :type Integer))
  (bind _discoveredtilesortingcost (`self.DiscoveredTileSortingCost`))
  (set `local.SortingCost` (`self.Get Tile Sorting Cost` TileData))
  (if (== (`KismetArrayLibrary.Array_Length` (`self.DiscoveredTileSortingCost`)) 0)
    (`KismetArrayLibrary.Array_Add` (`self.DiscoveredTileSortingCost`) (`local.SortingCost`) :!label _label)
    (`KismetArrayLibrary.Array_Add` (`self.DiscoveredTileIndexes`) (`.Index_10_021D3DFB40F95023808975A0CD205470` (break `/Game/Blueprints/Cores/Utility/S_PathFindingData` (`local.TileData`))))
    (elif (>= (`local.SortingCost`) (`|GetArrayItem` _discoveredtilesortingcost (`KismetArrayLibrary.Array_LastIndex` _discoveredtilesortingcost)))
      (goto _label)
      (else
        (for (_array_element _array_index) (`self.DiscoveredTileSortingCost`)
          (if (>= _array_element (`local.SortingCost`))
            (`KismetArrayLibrary.Array_Insert` (`self.DiscoveredTileSortingCost`) (`local.SortingCost`) _array_index)
            (`KismetArrayLibrary.Array_Insert` (`self.DiscoveredTileIndexes`) (`.Index_10_021D3DFB40F95023808975A0CD205470` (break `/Game/Blueprints/Cores/Utility/S_PathFindingData` (`local.TileData`))) _array_index)
            (break)))))))

(fn `IsDiagonal`
  (params (Index1 :type "IntPoint Structure") (Index2 :type "IntPoint Structure"))
  (returns (IsDiagonal :type Boolean))
  (bind _neighbors (`self.GetTileNeighbors` Index1))
  (return (not (`KismetArrayLibrary.Array_Contains` _neighbors Index2))))

(fn `IsInputDataValid`
  (returns (IsValid :type Boolean))
  (if (!= (`self.StartIndex`) (`self.TargetIndex`))
    (if (`/Game/Blueprints/Cores/Grid/BP_Grid.IsTileWalkable` (`self.Grid`) (`self.StartIndex`))
      (if (not (`self.ReturnReachableTiles`))
        (if (`/Game/Blueprints/Cores/Grid/BP_Grid.IsTileWalkable` (`self.Grid`) (`self.TargetIndex`))
          (if (<= (`self.GetMinimunCostBetweenTwoTiles` (`self.StartIndex`) (`self.TargetIndex`) (`self.IncludeDiagonals`)) (`self.MaxPathLength`))
            (if (not (`KismetSystemLibrary.IsValid` (`.UnitOnTile_17_296A43A74D08FB5B42D4D6A68D6A09A4` (break `/Game/Blueprints/Cores/Utility/S_TileData` (`BlueprintMapLibrary.Map_Find` (`/Game/Blueprints/Cores/Grid/BP_Grid.GridTiles` (`self.Grid`)) (`self.TargetIndex`))))))
              (return true)
              (else
                (return false)))
            (else
              (return false)))
          (else
            (return false)))
        (else
          (return true)))
      (else
        (return false)))
    (else
      (return false))))

(fn `PullCheapesTileOutOfDiscoveredList`
  (returns (TilePathData :type "/Game/Blueprints/Cores/Utility/S_PathFindingData Structure"))
  (locals (TileIndex :type "IntPoint Structure"))
  (set `local.TileIndex` (`|GetArrayItem` (`self.DiscoveredTileIndexes`)))
  (`KismetArrayLibrary.Array_Remove` (`self.DiscoveredTileSortingCost`))
  (`KismetArrayLibrary.Array_Remove` (`self.DiscoveredTileIndexes`))
  (`KismetArrayLibrary.Array_Add` (`self.AnalizeTileIndexes`) (`local.TileIndex`))
  (return (`BlueprintMapLibrary.Map_Find` (`self.PathFindingData`) (`local.TileIndex`))))

(fn `UserConstructionScript`)