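; BP_Grid is an actor that builds a square, hexagon or triangle tile grid in its construction script.
; SpawnGrid pulls mesh and material from DT_GridShapeData, snaps center and corner, then adds one InstancedStaticMesh instance per tile using shape-specific spacing, staggering and rotation.
; With environment use enabled, sphere traces snap tile heights to the ground and skip tiles that hit nothing.
; GetCursorLocationOnGrid is an unfinished stub.
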(fn `CalculateCenter&BottomLeft`
  (returns (Center :type "Vector Structure") (BottomLeft :type "Vector Structure"))
  (locals (SnapCenter :type "Vector Structure" :default (0.0 0.0 0.0)))
  (bind (_grid_tile_count_x _grid_tile_count_y) (break `IntPoint` (`self.Grid Tile Count`)))
  (bind (_grid_tile_size_x _grid_tile_size_y) (`KismetMathLibrary.BreakVector` (`self.Grid Tile Size`)))
  (bind (_grid_tile_size_x_2 _grid_tile_size_y_2) (`KismetMathLibrary.BreakVector` (`self.Grid Tile Size`)))
  (bind (_grid_tile_size_x_3 _grid_tile_size_y_3) (`KismetMathLibrary.BreakVector` (`self.Grid Tile Size`)))
  (bind (_returnvalue_x _returnvalue_y) (`KismetMathLibrary.BreakVector` (* (/ (- (`self.Grid Tile Count`) (`KismetMathLibrary.MakeVector2D` (`KismetMathLibrary.SelectFloat` 0.0 1.0 (`/Game/Blueprints/Cores/Utility/BFL_Utilities.IsIntEven` _grid_tile_count_x)) (`KismetMathLibrary.SelectFloat` 0.0 1.0 (`/Game/Blueprints/Cores/Utility/BFL_Utilities.IsIntEven` _grid_tile_count_y)))) (2.0 2.0)) (`KismetMathLibrary.MakeVector` _grid_tile_size_x_3 _grid_tile_size_y_3))))
  (switch `/Game/Blueprints/Cores/Grid/GridShapes/E_GridShape` (`self.Grid Shape`)
    (:`NewEnumerator1`
      ;[1 1 1] Comment
      (bind _output_get (set `local.SnapCenter` (`/Game/Blueprints/Cores/Utility/BFL_Utilities.SnapVectorToVector` (`self.Grid Center Location`) (* (`self.Grid Tile Size`) (1.5 1.0 1.0)))))
      (return _output_get (- _output_get (`/Game/Blueprints/Cores/Utility/BFL_Utilities.SnapVectorToVector` (* (/ (`self.Grid Tile Count`) (3.0 2.0)) (`KismetMathLibrary.MakeVector` _grid_tile_size_x_2 _grid_tile_size_y_2)) (* (`self.Grid Tile Size`) (1.5 1.0 1.0))))))
    (:`NewEnumerator2`
      ;[1 1 1] Comment
      (bind _output_get_2 (set `local.SnapCenter` (`/Game/Blueprints/Cores/Utility/BFL_Utilities.SnapVectorToVector` (`self.Grid Center Location`) (`self.Grid Tile Size`))))
      (return _output_get_2 (- _output_get_2 (`KismetMathLibrary.MakeVector` _returnvalue_x _returnvalue_y))))
    (:`NewEnumerator3`
      ;[1 1 1] Comment
      (bind _output_get_3 (set `local.SnapCenter` (`/Game/Blueprints/Cores/Utility/BFL_Utilities.SnapVectorToVector` (`self.Grid Center Location`) (* (`self.Grid Tile Size`) (2.0 1.0 1.0)))))
      (return _output_get_3 (- _output_get_3 (`/Game/Blueprints/Cores/Utility/BFL_Utilities.SnapVectorToVector` (* (/ (- (`self.Grid Tile Count`) (10.0 1.0)) (2.0 4.0)) (`KismetMathLibrary.MakeVector` _grid_tile_size_x _grid_tile_size_y)) (* (`self.Grid Tile Size`) (2.0 1.0 1.0))))))))

(fn `ClearInstances`
  (`InstancedStaticMeshComponent.ClearInstances` (`self.InstancedStaticMesh`)))

(fn `GetCursorLocationOnGrid`
  (params (PlayerIndex :type Integer)))

(fn `GetShapeData`
  (returns (ReturnValue :type "/Game/Blueprints/Cores/Grid/GridShapes/S_GridShapeData Structure"))
  (bind _returnvalue (`|GetEnumeratorNameAsString` (`self.Grid Shape`)))
  (bind _returnvalue_2 (`|GetDataTableRow` "/Game/Blueprints/Cores/Grid/GridShapes/DT_GridShapeData.DT_GridShapeData" (`KismetStringLibrary.Conv_StringToName` _returnvalue))
    (:`then`
      (return _returnvalue_2))
    (:`RowNotFound`
      (`KismetSystemLibrary.PrintString` (`KismetStringLibrary.Concat_StrStr` "Error - Shape Not Found -" _returnvalue)))))

(fn `GetTileLocationFromGridIndex`
  (params (GridIndex :type "IntPoint Structure"))
  (returns (TileLocation :type "Vector Structure"))
  (bind (_returnvalue_x _returnvalue_y) (`KismetMathLibrary.BreakVector2D` (* GridIndex (select `/Game/Blueprints/Cores/Grid/GridShapes/E_GridShape` (`self.Grid Shape`) :`NewEnumerator1` (0.75 0.5) :`NewEnumerator2` (1.0 1.0) :`NewEnumerator3` (1.0 0.5) :!type "Vector2D Structure"))))
  (return (+ (`self.Grid Bottom Left Corner Location`) (* (`self.Grid Tile Size`) (`KismetMathLibrary.MakeVector` _returnvalue_x _returnvalue_y)))))

(fn `GetTileRotationFromGridIndex`
  (params (GridIndex :type "IntPoint Structure"))
  (returns (TileRotation :type "Rotator Structure"))
  (bind (_gridindex_x _gridindex_y) (break `IntPoint` (`local.GridIndex`)))
  (if (`|EnumEquality` (`self.Grid Shape`) "NewEnumerator3")
    (return (`KismetMathLibrary.MakeRotator` 0.0 (+ (`KismetMathLibrary.SelectFloat` 180.0 0.0 (`/Game/Blueprints/Cores/Utility/BFL_Utilities.IsIntEven` _gridindex_x)) (`KismetMathLibrary.SelectFloat` 180.0 0.0 (`/Game/Blueprints/Cores/Utility/BFL_Utilities.IsIntEven` _gridindex_y)))))
    (else
      (return))))

(fn `SetGridOffsetFromGround`
  (params (Offset :type "Float (double-precision)"))
  (bind _output_get (set `self.GridOffsetFromGround` Offset))
  (`SceneComponent.K2_SetWorldLocation` (`self.InstancedStaticMesh`) (`KismetMathLibrary.MakeVector` 0.0 0.0 _output_get) false false))

(fn `SpawnGrid`
  (params (CenterLocation :type "Vector Structure") (TileSize :type "Vector Structure") (TileCount :type "IntPoint Structure") (Shape :type "/Game/Blueprints/Cores/Grid/GridShapes/E_GridShape Enum" :default "NewEnumerator0"))
  (locals (XIndex :type Integer) (YIndex :type Integer) (TileTransform :type "Transform Structure") (Index :type "IntPoint Structure"))
  (bind _instancedstaticmesh (`self.InstancedStaticMesh`))
  (bind (_grid_tile_count_x _grid_tile_count_y) (break `IntPoint` (`self.Grid Tile Count`)))
  (bind _index (`local.Index`))
  (bind _grid_tile_count_x_2 (break `IntPoint` (`self.Grid Tile Count`)))
  (bind (_grid_tile_count_x_3 _grid_tile_count_y_2) (break `IntPoint` (`self.Grid Tile Count`)))
  (bind (_meshsize _mesh _mesmaterial _flatmesh _flatbordermaterial) (break `/Game/Blueprints/Cores/Grid/GridShapes/S_GridShapeData` (`self.GetShapeData`)))
  (set `self.Grid Center Location` CenterLocation)
  (set `self.Grid Tile Size` TileSize)
  (set `self.Grid Tile Count` TileCount)
  (set `self.Grid Shape` Shape)
  (`self.ClearInstances`)
  (`StaticMeshComponent.SetStaticMesh` _instancedstaticmesh _flatmesh)
  (`PrimitiveComponent.SetMaterial` _instancedstaticmesh 0 _flatbordermaterial)
  (`self.SetGridOffsetFromGround` (`self.GridOffsetFromGround`))
  (bind (_center _bottomleft) (`self.CalculateCenter&BottomLeft`))
  (set `self.Grid Center Location` _center)
  (set `self.Grid Bottom Left Corner Location` _bottomleft)
  (for _index_2 (range _grid_tile_count_x_2)
    (set `local.XIndex` _index_2)
    (if (`|EnumInequality` (`self.Grid Shape`) "NewEnumerator1")
      (for _index_3 (range _grid_tile_count_y_2)
        (set `local.YIndex` _index_3)
        (set `local.Index` (make `IntPoint` (`local.XIndex`) (`local.YIndex`)) :!label _label)
        (bind _output_get (set `local.TileTransform` (`KismetMathLibrary.MakeTransform` (`self.GetTileLocationFromGridIndex` _index) (`self.GetTileRotationFromGridIndex` _index) (/ (`self.Grid Tile Size`) (`.MeshSize_2_395DE89842B358E49DC592ADA02F14A6` (break `/Game/Blueprints/Cores/Grid/GridShapes/S_GridShapeData` (`self.GetShapeData`)))))))
        (if (`self.UseEnvirontment`)
          (bind (_hitsomething _outlocation) (`self.TraceForGround` (.location _output_get)))
          (if _hitsomething
            (bind _output_get_2 (set `local.TileTransform` (`KismetMathLibrary.MakeTransform` _outlocation (.rotation _output_get) (.scale _output_get))))
            (`InstancedStaticMeshComponent.AddInstance` (`self.InstancedStaticMesh`) _output_get_2 false))
          (else
            (`InstancedStaticMeshComponent.AddInstance` (`self.InstancedStaticMesh`) (`local.TileTransform`) false))))
      (else
        (for _index_4 (range (`KismetMathLibrary.SelectInt` 0 1 (`/Game/Blueprints/Cores/Utility/BFL_Utilities.IsIntEven` (`local.XIndex`))) (* _grid_tile_count_y 2))
          (set `local.YIndex` _index_4)
          (`|ExecutionSequence`
            (:`then_0`
              (goto _label))
            (:`then_1`
              (`/Engine/EditorBlueprintResources/StandardMacros.IncrementInt` _index_4))))))))

(fn `TraceForGround`
  (params (Locaion :type "Vector Structure"))
  (returns (HitSomething :type Boolean) (OutLocation :type "Vector Structure"))
  (locals (Radius :type "Float (single-precision)" :default 0.0))
  (bind (_x _y) (`KismetMathLibrary.BreakVector3f` Locaion))
  (bind _grid_tile_size_x (`KismetMathLibrary.BreakVector` (`self.Grid Tile Size`)))
  (bind (_grid_tile_size_x_2 _grid_tile_size_y _grid_tile_size_z) (`KismetMathLibrary.BreakVector` (`self.Grid Tile Size`)))
  (set `local.Radius` (/ _grid_tile_size_x (`KismetMathLibrary.SelectFloat` 5.0 3.0 (`|EnumEquality` (`self.Grid Shape`) "NewEnumerator3"))))
  (bind _outhits (`KismetSystemLibrary.SphereTraceMulti` (+ Locaion (0.0 0.0 1000.0)) (- Locaion (0.0 0.0 1000.0)) (`local.Radius`) "TraceTypeQuery3"))
  (if (> (`KismetArrayLibrary.Array_Length` _outhits) 0)
    (return true (`KismetMathLibrary.MakeVector` _x _y (`KismetMathLibrary.GridSnap_Float` (- (`.Z` (`KismetMathLibrary.BreakVector3f` (`.Location` (`GameplayStatics.BreakHitResult` (`|GetArrayItem` _outhits))))) (`local.Radius`)) _grid_tile_size_z)))
    (else
      (return false Locaion))))

(fn `UserConstructionScript`
  (`self.SpawnGrid` (`self.K2_GetActorLocation`) (`self.Grid Tile Size`) (`self.Grid Tile Count`) (`self.Grid Shape`)))