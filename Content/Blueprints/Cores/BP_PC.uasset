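; BP_PC is a player controller for battle play that shows the mouse cursor, creates the battle HUD widget on BeginPlay and handles clicking to select units.
; Left click traces under the cursor on the Camera channel and, if the hit actor implements BPI_PlayerBase, stores it as SelectedUnit.
; Debug prints confirm a unit click or otherwise show the name of whatever was hit.
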(event `self.ReceiveBeginPlay`
  (set `self.bShowMouseCursor` true)
  (bind _returnvalue (`|CreateWidget` "/Game/UIs/CombatWidget/WBP_BattleHUD.WBP_BattleHUD_C"))
  (bind _output_get (set `self.BattleHUD` _returnvalue))
  (`UserWidget.AddToViewport` _output_get 0))

(event `Key|LeftMouseButton`
  (params (Key :type "Key Structure"))
  (bind (_bblockinghit _binitialoverlap _time _distance _location _impactpoint _normal _impactnormal _physmat _hitactor) (`GameplayStatics.BreakHitResult` (`self.GetHitResultUnderCursorByChannel` "TraceTypeQuery2")))
  (:`Pressed`
    (if (`KismetSystemLibrary.DoesImplementInterface` _hitactor "/Game/Blueprints/Characters/Old/BPI_PlayerBase.BPI_PlayerBase_C")
      (set `self.SelectedUnit` _hitactor)
      (`KismetSystemLibrary.PrintString` "unit clicked")
      (else
        (`KismetSystemLibrary.PrintString` (`KismetSystemLibrary.GetDisplayName` _hitactor))))))

(event `Key|RightMouseButton`
  (params (Key :type "Key Structure")))

(fn `UserConstructionScript`)